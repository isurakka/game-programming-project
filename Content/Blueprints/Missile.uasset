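; Homing missile actor that climbs, locks onto a random nearby Enemy and deals point damage on hit before destroying itself.
; A three-state Tick drives it: rise for a set time, sphere-overlap for enemies, then steer toward the chosen target.
; Steering interpolates the actor's up axis toward the target and sets physics velocity along it.
; A lifespan starts after the climb, and a lost target is never reacquired.
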(event `self.ReceiveBeginPlay`
  (`KismetSystemLibrary.Delay` (`self.GoUpDuration`))
  (set `self.State` 1)
  (`self.SetLifeSpan` 10.0))

(event `self.ReceiveTick`
  (params (DeltaSeconds :type "Float (single-precision)"))
  (switch `int` (`self.State`)
    (:`0`
      (`PrimitiveComponent.SetPhysicsLinearVelocity` (* (`self.GetActorUpVector`) (`self.GoUpSpeed`))))
    (:`1`
      (bind _outactors (`KismetSystemLibrary.SphereOverlapActors_NEW` (`self.K2_GetActorLocation`) (`self.TargetFindRadius`) (`|MakeArray` "ObjectTypeQuery3" :!type "EngineTypes.EObjectTypeQuery Enum") "/Game/Blueprints/AI/Enemy.Enemy_C"))
      (if (> (`KismetArrayLibrary.Array_Length` _outactors) 0)
        (`KismetArrayLibrary.Array_Shuffle` _outactors)
        (bind _asenemy (cast `/Game/Blueprints/AI/Enemy` (`KismetArrayLibrary.Array_Get` _outactors)))
        (set `self.Target` _asenemy)
        (set `self.State` 2)))
    (:`2`
      (`/Engine/EditorBlueprintResources/StandardMacros.IsValid` (`self.Target`)
        (:`Is Valid`
          (`self.SetActorRotation` (`KismetMathLibrary.RInterpTo` (`self.K2_GetActorRotation`) (`KismetMathLibrary.MakeRotFromZ` (- (`self.K2_GetActorLocation` (`self.Target`)) (`self.K2_GetActorLocation`))) DeltaSeconds (`self.RotationSpeed`)))
          (`PrimitiveComponent.SetPhysicsLinearVelocity` (`self.Mesh`) (* (`self.GetActorUpVector`) (`self.GoUpSpeed`)) false "None"))))))

(event `self.ReceiveHit`
  (params (MyComp :type "PrimitiveComponent Object Reference") (Other :type "Actor Object Reference") (OtherComp :type "PrimitiveComponent Object Reference") (bSelfMoved :type Boolean) (HitLocation :type "Object.Vector Structure") (HitNormal :type "Object.Vector Structure") (NormalImpulse :type "Object.Vector Structure") (Hit :type "EngineTypes.HitResult Structure (by ref)"))
  (`GameplayStatics.ApplyPointDamage` Other (`self.Damage`) (`KismetMathLibrary.NegateVector` HitNormal) Hit)
  (`self.K2_DestroyActor`))

(fn `UserConstructionScript`
  (`SceneComponent.SetRelativeScale3D` (`self.Mesh`) (0.5 0.5 0.5)))