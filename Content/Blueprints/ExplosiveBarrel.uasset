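; An explosive barrel actor that blows up when damage drains its health.
; Each AnyDamage event prints a debug string and subtracts the damage from Health, clamping it at zero.
; At zero health it spawns the Blueprint_Effect_Explosion actor at its own transform, ignoring collision, then destroys itself.
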(event `self.ReceiveAnyDamage`
  (params (Damage :type "Float (single-precision)") (DamageType :type "DamageType Object Reference") (InstigatedBy :type "Controller Object Reference") (DamageCauser :type "Actor Object Reference"))
  (bind _returnvalue (- (`self.Health`) Damage))
  (`KismetSystemLibrary.PrintString` "Hello")
  (if (< _returnvalue 0.0)
    (set `self.Health` 0.0)
    (else
      (set `self.Health` _returnvalue)))
  (if (== (`self.Health`) 0.0)
    (`|SpawnActorFromClass` "/Game/StarterContent/Blueprints/Blueprint_Effect_Explosion.Blueprint_Effect_Explosion_C" (`self.GetTransform`) true)
    (`self.K2_DestroyActor`)))

(fn `UserConstructionScript`)