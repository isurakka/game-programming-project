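; Health component that gives its owning actor hit points, broadcasts a die event and destroys the owner when health runs out.
; It binds to the owner's any-damage event to subtract health.
; A non-lethal hit saves each mesh component's materials, swaps them to a white flash material and plays a hit sound.
; Tick restores the saved materials after the flash duration, and repeat hits during a flash only restart the timer.
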(event `self.ReceiveInitializeComponent`
  (bind _output_get (set `self.Parent Actor` (`self.GetOwner`)))
  (add `Actor.OnTakeAnyDamage` _output_get (delegate `HealthComponent_damage`)))

(event `HealthComponent_damage`
  (params (Damage :type "Float (double-precision)" :default 0.0) (DamageType :type "DamageType Object Reference") (InstigatedBy :type "Controller Object Reference") (DamageCauser :type "Actor Object Reference"))
  (bind _output_get (set `self.Health` (- (`self.Health`) Damage)))
  (if (<= _output_get 0.0)
    (`self.OnDie`)
    (`Actor.K2_DestroyActor` (`self.Parent Actor`))
    (`KismetSystemLibrary.PrintString` "Hello")
    (elif (`self.OnWhiteTimer`)
      (set `self.WhiteTimer` 0.0)
      (else
        (set `self.OnWhiteTimer` true)
        (for _array_element (`Actor.K2_GetComponentsByClass` (`self.Parent Actor`) "/Script/Engine.MeshComponent")
          (`|ExecutionSequence`
            (:`then_0`
              (bind _returnvalue (`MeshComponent.GetMaterials` _array_element))
              (`KismetArrayLibrary.Array_Add` (`self.OriginalMaterials`) (make `/Game/Blueprints/AI/OldMaterialStruct` _array_element _returnvalue)))
            (:`then_1`
              (for (_ _array_index) _returnvalue
                (`PrimitiveComponent.SetMaterial` _array_element _array_index "/Game/Materials/BarrelWhite.BarrelWhite")))))
        (`GameplayStatics.PlaySoundAtLocation` (`self.Hitsound`) (`Actor.K2_GetActorLocation` (`self.Parent Actor`)))))))

(event `self.ReceiveTick`
  (params (DeltaSeconds :type "Float (single-precision)"))
  (if (`self.OnWhiteTimer`)
    (set `self.WhiteTimer` (+ (`self.WhiteTimer`) DeltaSeconds))
    (if (> (`self.WhiteTimer`) (`self.WhiteDuration`))
      (`|ExecutionSequence`
        (:`then_0`
          (for _array_element (`Actor.K2_GetComponentsByClass` (`self.Parent Actor`) "/Script/Engine.MeshComponent")
            (for _array_element_2 (`self.OriginalMaterials`)
              (if (== (`.Mesh_3_EA122BE042AD2B3D5BDC54915956D15F` (break `/Game/Blueprints/AI/OldMaterialStruct` _array_element_2)) _array_element)
                (set `self.TempOriginalMaterial` _array_element_2)
                (break)))
            (for (_ _array_index) (`MeshComponent.GetMaterials` _array_element)
              (`PrimitiveComponent.SetMaterial` _array_element _array_index (`KismetArrayLibrary.Array_Get` (`.Materials_6_A1383EEB431ECB73241B628BA69808D7` (break `/Game/Blueprints/AI/OldMaterialStruct` (`self.TempOriginalMaterial`))) _array_index))))
          (`KismetArrayLibrary.Array_Clear` (`self.OriginalMaterials`)))
        (:`then_1`
          (set `self.WhiteTimer` 0.0)
          (set `self.OnWhiteTimer` false))))))

(fn `Reset material`)