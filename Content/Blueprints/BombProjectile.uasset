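; Bomb projectile that takes one of two random game-mode colours at spawn and bursts into colour-matched swarm bullets on hit.
; BeginPlay picks the colour index and tints its particle system via CoopGameMode.
; Explode spawns tinted explosion effects, launches SwarmEnemyBullets carrying that colour and index, then destroys the actor.
; Bullet impulses come from rotating the normalised world location in yaw steps, rather than a forward vector.
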(event `self.ReceiveHit`
  (params (MyComp :type "PrimitiveComponent Object Reference") (Other :type "Actor Object Reference") (OtherComp :type "PrimitiveComponent Object Reference") (bSelfMoved :type Boolean) (HitLocation :type "Object.Vector Structure") (HitNormal :type "Object.Vector Structure") (NormalImpulse :type "Object.Vector Structure") (Hit :type "EngineTypes.HitResult Structure (by ref)"))
  (`self.Explode`))

(event `self.ReceiveBeginPlay`
  (`|ExecutionSequence`
    (:`then_0`
      (set `self.ColorIndex` (`KismetMathLibrary.RandomIntegerInRange` 0 1)))
    (:`then_1`
      (bind _ascoop_game_mode (cast `/Game/Blueprints/CoopGameMode` (`GameplayStatics.GetGameMode`)))
      (bind _color (`/Game/Blueprints/ColorChangingHelpers.GetColorForIndex` (`self.ColorIndex`) _ascoop_game_mode))
      (bind _output_get (set `self.CurrentColor` _color))
      (`ParticleSystemComponent.SetVectorParameter` (`self.ParticleSystem`) "ProjectileColor" (`KismetMathLibrary.Conv_LinearColorToVector` _output_get)))))

(event `self.ReceiveActorBeginOverlap`
  (params (OtherActor :type "Actor Object Reference")))

(event `self.ReceiveTick`
  (params (DeltaSeconds :type "Float (single-precision)")))

(fn `Explode`
  (bind _currentcolor (`self.CurrentColor`))
  (`|ExecutionSequence`
    (:`then_0`
      (bind _returnvalue (`GameplayStatics.SpawnEmitterAtLocation` "/Game/Enemies/Particles/PFX_EnemyExplosion.PFX_EnemyExplosion" (`self.K2_GetActorLocation`) (`self.K2_GetActorRotation`)))
      (`SceneComponent.SetWorldScale3D` _returnvalue (2.0 2.0 2.0))
      (`ParticleSystemComponent.SetVectorParameter` _returnvalue "EnemyColor" (`KismetMathLibrary.Conv_LinearColorToVector` _currentcolor))
      (`ActorComponent.Activate` false))
    (:`then_1`
      (bind _returnvalue_2 (`|SpawnActorFromClass` "/Game/Blueprints/Blueprint_Effect_Explosion.Blueprint_Effect_Explosion_C" (`self.GetTransform`)))
      (`self.SetActorScale3D` _returnvalue_2 (4.0 4.0 4.0))
      (set `/Game/Blueprints/Blueprint_Effect_Explosion.Blast color` _currentcolor _returnvalue_2)
      (`/Game/Blueprints/Blueprint_Effect_Explosion.Activate` _returnvalue_2))
    (:`then_2`
      (for _index (range 13)
        (bind _returnvalue_3 (`|SpawnActorFromClass` "/Game/Blueprints/SwarmEnemyBullet.SwarmEnemyBullet_C" (`self.GetTransform`)))
        (`|ExecutionSequence`
          (:`then_0`
            (bind _asmaterial_instance_dynamic (cast `MaterialInstanceDynamic` (`PrimitiveComponent.GetMaterial` _returnvalue_3 0)))
            (`MaterialInstanceDynamic.SetVectorParameterValue` _asmaterial_instance_dynamic "Color" (`self.CurrentColor`))
            (set `/Game/Blueprints/BulletProjectile.Color Index` (`self.ColorIndex`) _returnvalue_3))
          (:`then_1`
            (`PrimitiveComponent.AddImpulse` _returnvalue_3 (* (`KismetMathLibrary.Normal` (`KismetMathLibrary.GreaterGreater_VectorRotator` (`self.K2_GetActorLocation`) (`KismetMathLibrary.MakeRot` 0.0 (* _index 30.0)))) 1500.0) "None" true))))
      (`self.K2_DestroyActor`))))

(fn `UserConstructionScript`)