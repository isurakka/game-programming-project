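; Co-op game mode that tracks enemy kill progress for level advancement and creates ammo pickups.
; Shortly after BeginPlay it adds all Worm and Enemy actors to the level total; IncrementKilledEnemies returns whether the kill ratio meets the advance threshold.
; CreateAmmo picks a random weapon class from those in the world and spawns matching Ammo with its color and a random share of max capacity, scaling the mesh accordingly.
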(event EventTick
  (params (DeltaSeconds :type Float%20%28single-precision%29)))

(event EventBeginPlay
  (Utilities|FlowControl|Delay 0.2)
  (Utilities|FlowControl|Sequence
    (:then_0
      (bind _outactors (Actor|GetAllActorsOfClass "/Game/Blueprints/AI/Worm/Worm.Worm_C"))
      (CallFunction|IncrementTotalNumberOfEnemies (Utilities|Array|Length _outactors)))
    (:then_1
      (bind _outactors_2 (Actor|GetAllActorsOfClass "/Game/Blueprints/AI/Enemy.Enemy_C"))
      (CallFunction|IncrementTotalNumberOfEnemies (Utilities|Array|Length _outactors_2)))))

(fn ConstructionScript)

(fn CreateAmmo
  (bind _oneinstanceofweapons (LocalVariables|GetOneInstanceOfWeapons))
  (bind _ammogivepercentrange (LocalVariables|GetAmmoGivePercentRange))
  (bind _item (Utilities|Array|Get(acopy) _oneinstanceofweapons))
  (bind (_x _y) (Math|Vector2D|BreakVector2D _ammogivepercentrange))
  (bind _outactors (Actor|GetAllActorsOfClass "/Game/Blueprints/Weapons/Weapon.Weapon_C"))
  (for _array_element _outactors
    (bind _asweapon (Utilities|Casting|CastToWeaponClass (Utilities|GetClass _array_element)))
    (bind _returnvalue (Utilities|Array|AddUnique (LocalVariables|GetUniqueWeaponClasses) _asweapon))
    (if (>= _returnvalue 0)
      (Utilities|Array|Add _oneinstanceofweapons _array_element)))
  (Utilities|Array|Shuffle _oneinstanceofweapons)
  (bind _asweapon_2 (Utilities|Casting|CastToWeaponClass (Utilities|GetClass _item)))
  (bind _returnvalue_2 (Game|SpawnActorfromClass "/Game/Blueprints/Weapons/Ammo/Ammo.Ammo_C" (Math|Transform|MakeTransform "0, 0, 0") true 0))
  (Variables|/Game/Blueprints/Weapons/Ammo/Ammo.Ammo_C|SetForWeaponClass _returnvalue_2 _asweapon_2)
  (Default|SetColor _returnvalue_2 (Variables|/Game/Blueprints/Weapons/Weapon.Weapon_C|GetMainColor _item))
  (LocalVariables|SetAmmoGivePercent (Math|Random|RandomFloatinRange _x _y))
  (Default|SetAmmoCount _returnvalue_2 (Math|Float|Floor (Math|Float|Max(Float) (* (Variables|/Game/Blueprints/Weapons/Weapon.Weapon_C|GetMaxAmmoCount _item) (LocalVariables|GetAmmoGivePercent)) 1.0)) (* (LocalVariables|GetAmmoGivePercent) 3.0))
  (return _returnvalue_2))

(fn IncrementKilledEnemies
  (params (NewParam :type Integer :default 0))
  (Variables|Default|SetKilled%20enemies%20in%20level (+ (Variables|Default|GetKilled%20enemies%20in%20level) NewParam))
  (bind _current_kill_percentage (CallFunction|CalculateKillPercentage))
  (return (>= _current_kill_percentage (Variables|Default|GetPercentage%20of%20enemies%20to%20kill%20to%20advance))))

(fn IncrementTotalNumberOfEnemies
  (params (NewParam :type Integer :default 0))
  (Variables|Default|SetTotal%20number%20of%20enemies%20in%20level (+ (Variables|Default|GetTotal%20number%20of%20enemies%20in%20level) NewParam)))

(fn CalculateKillPercentage
  (bind _output_get (Variables|Default|SetPercentage%20of%20enemies%20killed%20in%20level (/ (Math|Conversions|ToFloat(Integer) (Variables|Default|GetKilled%20enemies%20in%20level)) (Math|Conversions|ToFloat(Integer) (Variables|Default|GetTotal%20number%20of%20enemies%20in%20level)))))
  (return _output_get))