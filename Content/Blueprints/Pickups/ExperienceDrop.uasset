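; ExperienceDrop is a physics-driven experience pickup that carries a drop value.
; On a hit, if the normalized velocity points mostly upward, it plays a bounce sound pitched by global time dilation and activates its particle system.
; The construction script sets a fixed half scale, and SetDropValue only stores the value because its scaling node is not wired in.
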(event `self.ReceiveHit`
  (params (MyComp :type "PrimitiveComponent Object Reference") (Other :type "Actor Object Reference") (OtherComp :type "PrimitiveComponent Object Reference") (bSelfMoved :type Boolean) (HitLocation :type "Object.Vector Structure") (HitNormal :type "Object.Vector Structure") (NormalImpulse :type "Object.Vector Structure") (Hit :type "EngineTypes.HitResult Structure (by ref)"))
  (bind _returnvalue (`PrimitiveComponent.GetPhysicsLinearVelocity` MyComp "None"))
  (if (> (.z (`KismetMathLibrary.Normal` _returnvalue)) 0.65)
    (`GameplayStatics.PlaySoundAtLocation` "/Game/Audio/Exp_bounce.Exp_bounce" (`self.K2_GetActorLocation`) 1.0 (`GameplayStatics.GetGlobalTimeDilation`))
    (`ActorComponent.Activate` (`self.ParticleSystem`) false)))

(event `self.ReceiveBeginPlay`)

(event `self.ReceiveActorBeginOverlap`
  (params (OtherActor :type "Actor Object Reference")))

(event `self.ReceiveTick`
  (params (DeltaSeconds :type "Float (single-precision)")))

(fn `Set drop value`
  (params (`Drop value` :type Integer :default 0))
  (set `self.Drop value` `Drop value`))

(fn `UserConstructionScript`
  (`SceneComponent.SetRelativeScale3D` (0.5 0.5 0.5)))