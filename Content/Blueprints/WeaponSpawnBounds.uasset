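; WeaponSpawnBounds is an actor Blueprint that spawns a random weapon at a given transform.
; SpawnOne shuffles the WeaponClasses array and spawns its first entry, even if that location is colliding, then always returns false.
; The event graph and construction script add no logic of their own, and nothing in this Blueprint calls SpawnOne.
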(event `self.ReceiveBeginPlay`
  (`parent.ReceiveBeginPlay`))

(event `self.ReceiveActorBeginOverlap`
  (params (OtherActor :type "Actor Object Reference"))
  (`parent.ReceiveActorBeginOverlap` null))

(event `self.ReceiveTick`
  (params (DeltaSeconds :type "Float (single-precision)"))
  (`parent.ReceiveTick` 0.0))

(fn `SpawnOne`
  (params (Transform :type "Object.Transform Structure"))
  (returns (Potato :type Boolean))
  (bind _weaponclasses (`self.WeaponClasses`))
  (`KismetArrayLibrary.Array_Shuffle` _weaponclasses)
  (`|SpawnActorFromClass` (`KismetArrayLibrary.Array_Get` _weaponclasses) Transform true)
  (return false))

(fn `UserConstructionScript`
  (`parent.UserConstructionScript`))