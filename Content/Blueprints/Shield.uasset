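; Shield actor scaled uniformly by its Radius, with a color that can be cycled.
; The construction script creates a dynamic material instance on the mesh and tints it from the local Colors array.
; NextColor gets the next index and color through helpers that take the Game Mode, updates the material and returns the color.
; GetColor and SetColor are stubs returning fixed values.
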(event `self.ReceiveBeginPlay`)

(fn `GetColor`
  (returns (index :type Integer))
  (return 0))

(fn `NextColor`
  (returns (Color :type "Object.LinearColor Structure"))
  (bind _returnvalue (`GameplayStatics.GetGameMode`))
  (bind _currentcolorindex (`self.CurrentColorIndex`))
  (set `self.CurrentColorIndex` (`/Game/Blueprints/ColorChangingHelpers.Get Next ColorIndex` _currentcolorindex _returnvalue))
  (bind _color (`/Game/Blueprints/ColorChangingHelpers.GetColorForIndex` _currentcolorindex _returnvalue))
  (`MaterialInstanceDynamic.SetVectorParameterValue` (`self.MaterialInstance`) "Color" _color)
  (return _color))

(fn `SetColor`
  (params (ColorIndex :type Integer))
  (returns (Nothing :type Boolean))
  (return false))

(fn `UserConstructionScript`
  (bind _radius (`self.Radius`))
  (bind _mesh (`self.Mesh`))
  (`self.SetActorRelativeScale3D` (`KismetMathLibrary.MakeVector` _radius _radius _radius))
  (bind _returnvalue (`PrimitiveComponent.CreateDynamicMaterialInstance` _mesh 0 (`PrimitiveComponent.GetMaterial` _mesh 0)))
  (set `self.MaterialInstance` _returnvalue)
  (`MaterialInstanceDynamic.SetVectorParameterValue` (`self.MaterialInstance`) "Color" (`KismetArrayLibrary.Array_Get` (`self.Colors`) (`self.CurrentColorIndex`))))