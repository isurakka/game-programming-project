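; Machine gun bullet actor that deals point damage to whatever it hits and then destroys itself.
; On begin play it waits out its lifetime, then self-destructs if still alive.
; Hit events apply bullet-type damage, deriving the hit direction from the reversed, normalized impulse.
; The construction script applies a uniform scale and swaps the first material for a dynamic instance without setting parameters.
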(event `self.ReceiveBeginPlay`
  (`KismetSystemLibrary.Delay` (`self.Lifetime`))
  (`self.K2_DestroyActor`))

(event `self.ReceiveHit`
  (params (MyComp :type "PrimitiveComponent Object Reference") (Other :type "Actor Object Reference") (OtherComp :type "PrimitiveComponent Object Reference") (bSelfMoved :type Boolean) (HitLocation :type "Object.Vector Structure") (HitNormal :type "Object.Vector Structure") (NormalImpulse :type "Object.Vector Structure") (Hit :type "EngineTypes.HitResult Structure (by ref)"))
  (`GameplayStatics.ApplyPointDamage` Other (`self.Damage`) (* (`KismetMathLibrary.Normal` NormalImpulse) -1.0) Hit null self "/Game/Blueprints/BulletDamageType.BulletDamageType_C")
  (`self.K2_DestroyActor`))

(fn `UserConstructionScript`
  (bind _scale (`self.Scale`))
  (`self.SetActorRelativeScale3D` (`KismetMathLibrary.MakeVector` _scale _scale _scale))
  (bind _returnvalue (`KismetMaterialLibrary.CreateDynamicMaterialInstance` (`PrimitiveComponent.GetMaterial` 0)))
  (`PrimitiveComponent.SetMaterial` 0 _returnvalue))