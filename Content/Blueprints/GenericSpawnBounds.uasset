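; Generic trigger-volume spawner that, on the first actor overlap, spawns a batch at random points and rotations inside its box, then destroys itself.
; SpawnOne is an empty stub returning false, apparently for child Blueprints to override with the actual spawn.
; CalculateSpawnCount scales the base Count by the CoopGameMode player count, weighting extra players by PlayerMultiplier.
; The construction script sizes the box uniformly from SpawnBoxScaleMultiplier.
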(event EventActorBeginOverlap
  (params (OtherActor :type Actor%20Object%20Reference))
  (if (not (Variables|Default|GetSpawned))
    (Variables|Default|SetSpawned true)
    (Utilities|FlowControl|Sequence
      (:then_0
        (bind _count (CallFunction|CalculateSpawnCount))
        (for _index (range 1 _count)
          (CallFunction|SpawnOne (Math|Transform|MakeTransform (Math|Random|RandomPointinBoundingBox (Transformation|GetWorldLocation) (Components|Box|GetScaledBoxExtent)) (Math|Random|RandomRotator true)))))
      (:then_1
        (Actor|DestroyActor)))))

(fn ConstructionScript
  (bind _spawnboxscalemultiplier (Variables|Default|GetSpawnBoxScaleMultiplier))
  (Transformation|SetRelativeScale3D (Math|Vector|MakeVector _spawnboxscalemultiplier _spawnboxscalemultiplier _spawnboxscalemultiplier)))

(fn SpawnOne
  (params (Transform :type Transform))
  (return false))

(fn CalculateSpawnCount
  (bind _count (Variables|Default|GetCount))
  (bind _ascoop_game_mode (Utilities|Casting|CastToCoopGameMode (Game|GetGameMode)))
  (if (> (Variables|/Game/Blueprints/CoopGameMode.CoopGameMode_C|GetNumber%20of%20players _ascoop_game_mode) 1)
    (LocalVariables|SetRetCount (+ _count (Math|Float|Ceil (* (* _count (- (Variables|/Game/Blueprints/CoopGameMode.CoopGameMode_C|GetNumber%20of%20players _ascoop_game_mode) 1)) (Variables|Default|GetPlayerMultiplier)))))
    (else
      (LocalVariables|SetRetCount (* (Variables|/Game/Blueprints/CoopGameMode.CoopGameMode_C|GetNumber%20of%20players _ascoop_game_mode) _count))))
  (return (LocalVariables|GetRetCount)))