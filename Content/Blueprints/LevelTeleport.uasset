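; Level exit teleporter that triggers the co-op game mode's level transition after a TopdownPlayer stays inside its capsule for a short charge time.
; Overlap starts named timers for the teleport and its sound, plus a timeline ramping rotation speed, light intensity and ambient sound pitch.
; Leaving the capsule halts both timers and reverses the timeline to wind the effects down.
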(event `self.ReceiveBeginPlay`)

(event `self.ReceiveActorBeginOverlap`
  (params (OtherActor :type "Actor Object Reference")))

(event `self.ReceiveTick`
  (params (DeltaSeconds :type "Float (single-precision)")))

(event `self.Capsule.OnComponentBeginOverlap`
  (params (OtherActor :type "Actor Object Reference") (OtherComp :type "PrimitiveComponent Object Reference") (OtherBodyIndex :type Integer) (bFromSweep :type Boolean) (SweepResult :type "EngineTypes.HitResult Structure (by ref)"))
  (cast `/Game/Blueprints/Player/TopdownPlayer` OtherActor)
  (`KismetSystemLibrary.K2_SetTimer` null "Teleport" 2.8)
  (`KismetSystemLibrary.K2_SetTimer` null "PlayTeleportSound" 2.6)
  (bind (_direction _rotationrate _lightintensity _soundpitch) (`Timeline|TeleportCharging` :!label _label)
    (:`Update`
      (set `RotatingMovementComponent.RotationRate` (`KismetMathLibrary.MakeRot` 0.0 _rotationrate) (`self.RotatingMovement`))
      (`LightComponent.SetIntensity` (`self.PointLight`) _lightintensity)
      (`AudioComponent.SetPitchMultiplier` (`self.AmbientSound`) _soundpitch))))

(event `self.Capsule.OnComponentEndOverlap`
  (params (OtherActor :type "Actor Object Reference") (OtherComp :type "PrimitiveComponent Object Reference") (OtherBodyIndex :type Integer))
  (cast `/Game/Blueprints/Player/TopdownPlayer` OtherActor)
  (`KismetSystemLibrary.K2_PauseTimer` null "Teleport")
  (`KismetSystemLibrary.K2_PauseTimer` null "PlayTeleportSound")
  (`KismetSystemLibrary.K2_ClearTimer` null "Teleport")
  (goto _label :!via `Reverse`))

(fn `PlayTeleportSound`
  (`AudioComponent.Play` 0.0))

(fn `Teleport`
  (`/Game/Blueprints/CoopGameMode.Initiate level transition` (cast `/Game/Blueprints/CoopGameMode` (`GameplayStatics.GetGameMode`) :!pure true)))

(fn `UserConstructionScript`)