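; Lightning gun weapon that fires branching chain lightning, with chain depth set by its level.
; Each shot runs ForkLightning in waves, with each hit seeding the next, a shared ignore list and per-wave forks, cone width and damage.
; ChainLightning damages the closest overlapped actor inside a dot-product cone and draws a color-indexed beam, aiming at a random point when the first wave misses.
; AutoGetLocation lets targets override their aim point through a CustomLocationGetter component.
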(event Custom|OnShoot
  (params (NewParam :type Integer :default 0))
  (bind _localchainstarts (Variables|Default|GetLocalChainStarts))
  (bind _localchaindirs (Variables|Default|GetLocalChainDirs))
  (bind _localchainignore (Variables|Default|GetLocalChainIgnore))
  (bind _localchainstarts_2 (Variables|Default|GetLocalChainStarts))
  (bind _localchaindirs_2 (Variables|Default|GetLocalChainDirs))
  (bind _newlocalchainstarts (Variables|Default|GetNewLocalChainStarts))
  (bind _newlocalchaindirs (Variables|Default|GetNewLocalChainDirs))
  (Variables|Default|SetColorIndex NewParam)
  (Audio|PlaySoundatLocation "/Game/Audio/lightning_zap.lightning_zap" (Transformation|GetActorLocation) 1.0 (Class|GameplayStatics|GetGlobalTimeDilation))
  (bind (_world_location _world_direction) (CallFunction|GetShootLocation))
  (CallFunction|GetPawn)
  (Utilities|FlowControl|Sequence
    (:then_0
      (bind _level (CallFunction|GetLevel))
      (switch int _level
        (:0
          _)
        (:1
          _)
        (:2
          _))
      (Utilities|Array|Clear _localchainstarts)
      (Utilities|Array|Add _localchainstarts _world_location)
      (Utilities|Array|Clear _localchaindirs)
      (Utilities|Array|Add _localchaindirs _world_direction)
      (Utilities|Array|Clear (Variables|Default|GetNewLocalChainStarts))
      (Utilities|Array|Clear (Variables|Default|GetNewLocalChainDirs))
      (Utilities|Array|Clear _localchainignore)
      (bind _index (Utilities|FlowControl|ForLoopwithBreak 0 (- (Utilities|Array|Get(acopy) (Variables|Default|GetChainsPerLevel) _level) 1))
        (:LoopBody
          (Utilities|FlowControl|Sequence
            (:then_0
              (for _array_element _newlocalchainstarts
                (Utilities|Array|Add (Variables|Default|GetLocalChainStarts) _array_element))
              (Utilities|Array|Clear _newlocalchainstarts))
            (:then_1
              (for _array_element_2 _newlocalchaindirs
                (Utilities|Array|Add (Variables|Default|GetLocalChainDirs) _array_element_2))
              (Utilities|Array|Clear _newlocalchaindirs))
            (:then_2
              (bind (_array_element_3 _array_index) (Utilities|Array|ForEachLoopwithBreak _localchainstarts_2)
                (:LoopBody
                  (bind (_hitpositions _hitdirections _hits) (CallFunction|ForkLightning (Utilities|Array|Get(acopy) (Variables|Default|GetForksPerChain) _index) _array_element_3 (Utilities|Array|Get(acopy) _localchaindirs_2 _array_index) NewParam _localchainignore (* (Variables|Default|GetBaseDamage) (Math|Conversions|ToFloat(Integer) (- 3 (+ _index 1)))) (Utilities|Array|Get(acopy) (Variables|Default|GetDotPerChain) _index) (== _index 0)))
                  (Utilities|FlowControl|Sequence
                    (:then_0
                      (for _array_element_4 _hits
                        (Utilities|IsValid _array_element_4
                          (:Is%20Valid
                            (Utilities|Array|Add (Variables|Default|GetLocalChainIgnore) _array_element_4)))))
                    (:then_1
                      (for _array_element_5 _hitpositions
                        (Utilities|Array|Add (Variables|Default|GetNewLocalChainStarts) _array_element_5)))
                    (:then_2
                      (for _array_element_6 _hitdirections
                        (Utilities|Array|Add (Variables|Default|GetNewLocalChainDirs) _array_element_6)))))
                (:Completed
                  (Utilities|Array|Clear _localchainstarts_2)
                  (Utilities|Array|Clear _localchaindirs_2))))))))))

(event EventBeginPlay
  (EventDispatchers|AssignShoot (delegate Custom|OnShoot)))

(fn ConstructionScript
  (|CallParentFunction)
  (Transformation|SetRelativeScale3D (Variables|Default|GetWeaponMeshComponent) "0.600000,0.600000,0.600000")
  (bind _returnvalue (Rendering|Material|CreateDynamicMaterialInstance "/Game/Materials/SimpleColor.SimpleColor" :!class /Script/Engine.KismetMaterialLibrary))
  (Rendering|Material|SetVectorParameterValue _returnvalue "Color" (Variables|Default|GetMainColor) :!class /Script/Engine.MaterialInstanceDynamic)
  (Rendering|Material|SetMaterial (Variables|Default|GetWeaponMeshComponent) 1 _returnvalue))

(fn ChainLightning
  (params (StartLocation :type Vector :default "0, 0, 0") (Direction :type Vector :default "0, 0, 0") (ColorIndex :type Integer :default 0) (Ignore :type Array%20of%20Actor%20Object%20References) (ChainToNothing :type Boolean :default false) (Damage :type Float%20%28single-precision%29 :default 0.0) (DotMin :type Float%20%28single-precision%29 :default 0.0))
  (bind _returnvalue (AddComponent|AddParticleSystemComponent false))
  (bind _color (CallFunction|GetColorforIndex ColorIndex (Game|GetGameMode)))
  (Effects|Components|ParticleSystem|SetColorParameter _returnvalue "Color" (Class|KismetMathLibrary|HSVtoRGB (.H (Math|Color|RGBtoHSV(LinearColor) _color)) (- (.S (Math|Color|RGBtoHSV(LinearColor) _color)) 0.1) (.V (Math|Color|RGBtoHSV(LinearColor) _color)) (.A (Math|Color|RGBtoHSV(LinearColor) _color))))
  (Utilities|FlowControl|Sequence
    (:then_0
      (Effects|Components|ParticleSystem|SetTemplate _returnvalue "/Game/Particles/LightningBeam.LightningBeam")
      (Class|ParticleSystemComponent|SetBeamSourcePoint _returnvalue 0 StartLocation)
      (bind _outactors (Class|KismetSystemLibrary|SphereOverlapActorsNEW StartLocation (Variables|Default|GetRange) (Utilities|Array|MakeArray "ObjectTypeQuery9") "/Script/Engine.Actor" Ignore))
      (for _array_element _outactors
        (if (> (Math|Vector|DotProduct (Math|Vector|Normalize (- (CallFunction|AutoGetLocation _array_element) StartLocation)) (Math|Vector|Normalize Direction)) DotMin)
          (Utilities|IsValid (LocalVariables|GetClosest)
            (:Is%20Valid
              (if (< (Math|Vector|VectorLength (- (CallFunction|AutoGetLocation _array_element) StartLocation)) (Math|Vector|VectorLength (- (CallFunction|AutoGetLocation (LocalVariables|GetClosest)) StartLocation)))
                (LocalVariables|SetClosest _array_element :!label _label)))
            (:Is%20Not%20Valid
              (goto _label)))))
      (Utilities|FlowControl|Sequence
        (:then_0
          (Utilities|IsValid (LocalVariables|GetClosest)
            (:Is%20Valid
              (Utilities|FlowControl|Sequence
                (:then_0
                  (LocalVariables|SetBeamTarget (CallFunction|AutoGetLocation (LocalVariables|GetClosest))))
                (:then_1
                  (Game|Damage|ApplyDamage (LocalVariables|GetClosest) Damage 0 self))))
            (:Is%20Not%20Valid
              (if ChainToNothing
                (LocalVariables|SetBeamTarget (+ (+ StartLocation (* Direction (- (Variables|Default|GetRange) (Variables|Default|GetRandomRadiusNoTarget)))) (* (Math|Random|RandomUnitVector) (Variables|Default|GetRandomRadiusNoTarget))))
                (else
                  (Rendering|SetVisibility _returnvalue false false)
                  (Components|DestroyComponent _returnvalue))))))
        (:then_1
          (Class|ParticleSystemComponent|SetBeamTargetPoint _returnvalue 0 (LocalVariables|GetBeamTarget))
          (return (LocalVariables|GetBeamTarget) (LocalVariables|GetClosest) (Math|Vector|Normalize (- (LocalVariables|GetBeamTarget) StartLocation))))))))

(fn ForkLightning
  (params (Branches :type Integer :default 0) (Start :type Vector :default "0, 0, 0") (Direction :type Vector :default "0, 0, 0") (ColorIndex :type Integer :default 0) (Ignore :type Array%20of%20Actor%20Object%20References) (Damage :type Float%20%28single-precision%29 :default 0.0) (DotMin :type Float%20%28single-precision%29 :default 0.0) (Chain%20to%20Nothing :type Boolean :default false))
  (Utilities|FlowControl|ForLoopwithBreak 0 Branches :!label _label
    (:LoopBody
      (bind (_hitpos _hit _hitdir) (CallFunction|ChainLightning Start Direction ColorIndex Ignore Chain%20to%20Nothing Damage DotMin))
      (Utilities|IsValid _hit
        (:Is%20Valid
          (Utilities|Array|Add (LocalVariables|GetLocalHits) _hit)
          (Utilities|Array|Add Ignore _hit)
          (Utilities|Array|Add (LocalVariables|GetLocalHitPositions) _hitpos)
          (Utilities|Array|Add (LocalVariables|GetLocalHitDirections) _hitdir))
        (:Is%20Not%20Valid
          (goto _label Break))))
    (:Completed
      (return (LocalVariables|GetLocalHitPositions) (LocalVariables|GetLocalHitDirections) (LocalVariables|GetLocalHits)))))

(fn AutoGetLocation
  (params (Actor :type Actor%20Object%20Reference))
  (bind _returnvalue (Actor|GetComponentsByClass Actor "/Game/Blueprints/CustomLocationGetter.CustomLocationGetter_C"))
  (if (> (Utilities|Array|Length _returnvalue) 0)
    (bind _customlocation (Default|GetCustomLocation (Utilities|Array|Get(acopy) _returnvalue)))
    (LocalVariables|SetRetLocation _customlocation)
    (else
      (LocalVariables|SetRetLocation (Transformation|GetActorLocation Actor))))
  (return (LocalVariables|GetRetLocation)))

(fn GetColorIndex
  (return (Variables|Default|GetColorIndex)))