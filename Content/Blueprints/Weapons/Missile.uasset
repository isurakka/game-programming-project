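; Missile projectile that wobbles along its up axis, deals point damage on hit, spawns an explosion and destroys itself.
; Tick sets physics velocity and eases rotation toward a periodically re-rolled random orientation.
; After a launch delay, homing missiles pick a random nearby Enemy and also steer toward it, searching again if it becomes invalid.
; A chance-based malfunction, rolled at BeginPlay, can cut homing, leaving only the random flight.
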(event `self.ReceiveTick`
  (params (DeltaSeconds :type "Float (single-precision)"))
  (bind _randomrotcurrent (`self.RandomRotCurrent`))
  (`|ExecutionSequence`
    (:`then_0`
      (set `self.LivedFor` (+ (`self.LivedFor`) DeltaSeconds)))
    (:`then_1`
      (`|ExecutionSequence`
        (:`then_0`
          (set `self.RandomRotCurrent` (+ _randomrotcurrent DeltaSeconds)))
        (:`then_1`
          (if (>= _randomrotcurrent (`self.RandomRotDuration`))
            (set `self.RandomRotCurrent` 0.0)
            (bind _target (`self.GetNewRandomRotation`))
            (set `self.RandomRotTarget` _target)))
        (:`then_2`
          (`self.SetActorRotation` (`KismetMathLibrary.RInterpTo` (`self.K2_GetActorRotation`) (`self.RandomRotTarget`) DeltaSeconds (`self.RandomRotSpeed`)))
          (`self.GoForward`))
        (:`then_4`
          (if (not (and (`self.GoingToMalfunction`) (>= (`self.LivedFor`) (`self.MalfunctionTime`))))
            (`|ExecutionSequence`
              (:`then_1`
                (if (`self.Homing`)
                  (switch `int` (`self.State`)
                    (:`1`
                      (`PrimitiveComponent.SetPhysicsLinearVelocity` (* (`self.GetActorUpVector`) (`self.GoUpSpeed`)))
                      (bind _outactors (`KismetSystemLibrary.SphereOverlapActors_NEW` (`self.K2_GetActorLocation`) (`self.TargetFindRadius`) (`|MakeArray` "ObjectTypeQuery3" :!type "EngineTypes.EObjectTypeQuery Enum") "/Game/Blueprints/AI/Enemy.Enemy_C"))
                      (if (> (`KismetArrayLibrary.Array_Length` _outactors) 0)
                        (`KismetArrayLibrary.Array_Shuffle` _outactors)
                        (bind _asenemy (cast `/Game/Blueprints/AI/Enemy` (`KismetArrayLibrary.Array_Get` _outactors)))
                        (set `self.Target` _asenemy)
                        (set `self.State` 2)))
                    (:`2`
                      (`/Engine/EditorBlueprintResources/StandardMacros.IsValid` (`self.Target`)
                        (:`Is Valid`
                          (`self.SetActorRotation` (`KismetMathLibrary.RInterpTo` (`self.K2_GetActorRotation`) (`KismetMathLibrary.MakeRotFromZ` (- (`self.K2_GetActorLocation` (`self.Target`)) (`self.K2_GetActorLocation`))) DeltaSeconds (`self.RotationSpeed`)))
                          (`PrimitiveComponent.SetPhysicsLinearVelocity` (`self.Mesh`) (* (`self.GetActorUpVector`) (`self.GoUpSpeed`)) false "None"))
                        (:`Is Not Valid`
                          (set `self.State` 1))))))))))))))

(event `self.ReceiveBeginPlay`
  (bind _returnvalue (>= (`self.MalfunctionChance`) (`KismetMathLibrary.RandomFloatInRange` 0.0 1.0)))
  (`|ExecutionSequence`
    (:`then_0`
      (bind _target (`self.GetNewRandomRotation`))
      (set `self.RandomRotTarget` _target)
      (`KismetSystemLibrary.Delay` (`self.GoUpDuration`))
      (set `self.State` 1))
    (:`then_1`
      (set `self.GoingToMalfunction` _returnvalue)
      (if _returnvalue
        (set `self.MalfunctionTime` (`KismetMathLibrary.RandomFloatInRange` (`self.MalfunctionMinLife`) (`KismetMathLibrary.FMin` (`self.GetLifeSpan`) (`self.MalfunctionMaxTime`))))))))

(event `self.ReceiveHit`
  (params (MyComp :type "PrimitiveComponent Object Reference") (Other :type "Actor Object Reference") (OtherComp :type "PrimitiveComponent Object Reference") (bSelfMoved :type Boolean) (HitLocation :type "Object.Vector Structure") (HitNormal :type "Object.Vector Structure") (NormalImpulse :type "Object.Vector Structure") (Hit :type "EngineTypes.HitResult Structure (by ref)"))
  (`GameplayStatics.ApplyPointDamage` Other (`self.Damage`) (`KismetMathLibrary.NegateVector` HitNormal) Hit null self)
  (`|SpawnActorFromClass` "/Game/Blueprints/Blueprint_Effect_Explosion.Blueprint_Effect_Explosion_C" (`KismetMathLibrary.MakeTransform` HitLocation (`self.K2_GetActorRotation`) (0.7 0.7 0.7)) true)
  (`self.K2_DestroyActor`))

(fn `GetColorIndex`
  (returns (ColorIndex :type Integer))
  (return (`self.ColorIndex`)))

(fn `GetNewRandomRotation`
  (returns (Target :type "Object.Rotator Structure"))
  (return (`KismetMathLibrary.MakeRotFromYZ` (* (`self.GetActorForwardVector`) (`KismetMathLibrary.RandomFloatInRange` -1.0 1.0)) (* (`self.GetActorRightVector`) (`KismetMathLibrary.RandomFloatInRange` -1.0 1.0)))))

(fn `GoForward`
  (`PrimitiveComponent.SetPhysicsLinearVelocity` (`self.Mesh`) (* (`self.GetActorUpVector`) (`self.GoUpSpeed`)) false "None"))

(fn `RotateRandom`)

(fn `SetColor`
  (params (ColorIndex :type Integer :default 0))
  (`/Game/Blueprints/ColorChangingHelpers.GetColorForIndex` ColorIndex (`GameplayStatics.GetGameMode`)))

(fn `UserConstructionScript`
  (`SceneComponent.SetRelativeScale3D` (`self.Mesh`) (0.5 0.5 0.5))
  (bind _returnvalue (`KismetMaterialLibrary.CreateDynamicMaterialInstance` (`PrimitiveComponent.GetMaterial` (`self.Mesh`) 0)))
  (`PrimitiveComponent.SetMaterial` 0 _returnvalue)
  (set `self.MeshMaterial` _returnvalue))