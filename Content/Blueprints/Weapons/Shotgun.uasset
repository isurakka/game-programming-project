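; Shotgun weapon that fires a fan of color-coded ShotgunProjectiles when its bound shoot event triggers.
; OnShoot spreads the shots around the Z axis with randomized angle steps, and the second level makes them bounce.
; CreateBullet spawns each projectile, launches it by impulse, orients it to the force, and tints its dynamic material with the CoopGameMode color for the shooter's index.
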(event `self.ReceiveBeginPlay`
  (add `self.Shoot` (delegate `onShoot`)))

(event `onShoot` :!signature `self.Shoot`
  (params (NewParam :type Integer))
  (bind (_world_location _world_direction) (`self.GetShootLocation`))
  (`self.GetPawn`)
  (bind _level (`self.GetLevel`))
  (switch `int` _level
    (:`0`
      ;[1 1 1] Level 1
      (for _index (range -3 3)
        (bind _returnvalue (`KismetMathLibrary.Conv_VectorToTransform` _world_location))
        (`self.Create bullet` _returnvalue NewParam (* (`KismetMathLibrary.Normal` (`KismetMathLibrary.RotateAngleAxis` _world_direction (`KismetMathLibrary.Conv_IntToDouble` (* _index (`KismetMathLibrary.RandomIntegerInRange` 8 12))) (0.0 0.0 1.0))) 3000.0))))
    (:`1`
      ;[1 1 1] Level 1
      (for _index_2 (range -3 3)
        (`self.Create bullet` _returnvalue NewParam (* (`KismetMathLibrary.Normal` (`KismetMathLibrary.RotateAngleAxis` _world_direction (`KismetMathLibrary.Conv_IntToDouble` (* _index_2 (`KismetMathLibrary.RandomIntegerInRange` 8 12))) (0.0 0.0 1.0))) 3000.0) true)))))

(event `self.ReceiveActorBeginOverlap`
  (params (OtherActor :type "Actor Object Reference")))

(event `self.ReceiveTick`
  (params (DeltaSeconds :type "Float (single-precision)"))
  (`parent.ReceiveTick` 0.0))

(fn `Create bullet`
  (params (Transform :type "Object.Transform Structure") (`Color Index` :type Integer :default 0) (Force :type "Object.Vector Structure" :default (0.0 0.0 0.0)) (Bounce :type Boolean))
  (`|ExecutionSequence`
    (:`then_0`
      (bind _returnvalue (`|SpawnActorFromClass` "/Game/Blueprints/Weapons/ShotgunProjectile.ShotgunProjectile_C" Transform true))
      (`PrimitiveComponent.AddImpulse` _returnvalue Force "None" true)
      (set `/Game/Blueprints/Weapons/ShotgunProjectile.Bounce` Bounce _returnvalue))
    (:`then_1`
      (`self.SetActorRotation` _returnvalue (`KismetMathLibrary.MakeRotFromZ` Force)))
    (:`then_2`
      (bind _asmaterial_instance_dynamic (cast `MaterialInstanceDynamic` (`PrimitiveComponent.GetMaterial` _returnvalue 0)))
      (bind _ascoop_game_mode (cast `/Game/Blueprints/CoopGameMode` (`GameplayStatics.GetGameMode`)))
      (bind _color (`/Game/Blueprints/ColorChangingHelpers.GetColorForIndex` `Color Index` _ascoop_game_mode))
      (`MaterialInstanceDynamic.SetVectorParameterValue` _asmaterial_instance_dynamic "Color" _color)
      (set `/Game/Blueprints/BulletProjectile.Color Index` `Color Index` _returnvalue))))

(fn `UserConstructionScript`
  (`parent.UserConstructionScript`))