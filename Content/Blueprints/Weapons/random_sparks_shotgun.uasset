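; Shotgun sparks actor that fires a one-off burst of particles, sound and light after a random delay.
; Tick feeds a Delay of random length, which then activates Effect and Sound and restarts the BrightnessControl timeline that animates the Flash light's intensity.
; The actor destroys itself when the particle system finishes, though the Tick-driven Delay can retrigger until then.
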(event `self.ReceiveTick`
  (params (DeltaSeconds :type "Float (single-precision)"))
  ;[1 1 1] Creating a random delay
  (`KismetSystemLibrary.Delay` (`KismetMathLibrary.RandomFloatInRange` 1.2 4.0))
  ;[1 1 1] Activating Particles and Sound
  (`ActorComponent.Activate` (`self.Effect`) false)
  (`ActorComponent.Activate` (`self.Sound`) false)
  ;[1 1 1] Activating lights with brightness animation
  (bind (_direction _intensity) (`Timeline|Brightness control` :!via `PlayFromStart`)
    (:`Update`
      (`LightComponent.SetIntensity` (`self.flash`) _intensity))))

(event `self.Effect.OnSystemFinished`
  (params (PSystem :type "ParticleSystemComponent Object Reference"))
  (`self.K2_DestroyActor` self))

(fn `UserConstructionScript`)