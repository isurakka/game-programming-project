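; Machine gun weapon that fires colored MachineGunBullet projectiles whenever its Shoot event fires.
; The weapon level selects one, three or five bullets, fanned around Z by angles from two timelines started at BeginPlay.
; CreateBullet spawns each bullet, launches it by velocity-change impulse, orients it and tints it via the CoopGameMode color index.
; Each bullet also plays an attached shot sound pitched by global time dilation.
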(event `self.ReceiveBeginPlay`
  (add `self.Shoot` (delegate `OnShoot`))
  (`|ExecutionSequence`
    (:`then_0`
      ;[1 1 1] Level 2
      (bind (_direction _angle) (`Timeline|ShootAngle`)))
    (:`then_1`
      ;[1 1 1] Level 3
      (bind (_direction_2 _angle1 _angle2) (`Timeline|ShootAngleLevel3`)))))

(event `OnShoot` :!signature `self.Shoot`
  (params (NewParam :type Integer :default 0))
  (bind (_world_location _world_direction) (`self.GetShootLocation`))
  (`self.GetPawn`)
  (`|ExecutionSequence`
    (:`then_0`
      (bind _level (`self.GetLevel`))
      (switch `int` _level
        (:`0`
          (bind _returnvalue (* _world_direction (`self.Bullet speed`)))
          (bind _returnvalue_2 (`KismetMathLibrary.MakeTransform` _world_location))
          ;[1 1 1] Level 1
          (`self.CreateBullet` _returnvalue _returnvalue_2 NewParam :!label _label))
        (:`1`
          ;[1 1 1] Level 2
          (`|ExecutionSequence`
            (:`then_0`
              (goto _label))
            (:`then_1`
              (`self.CreateBullet` (`KismetMathLibrary.RotateAngleAxis` _returnvalue (stale `self.ReceiveBeginPlay` _angle) (0.0 0.0 1.0)) _returnvalue_2 NewParam))
            (:`then_2`
              (`self.CreateBullet` (`KismetMathLibrary.RotateAngleAxis` _returnvalue (* (stale `self.ReceiveBeginPlay` _angle) -1.0) (0.0 0.0 1.0)) _returnvalue_2 NewParam))))
        (:`2`
          ;[1 1 1] Level 3
          (`|ExecutionSequence`
            (:`then_0`
              (`self.CreateBullet` (`KismetMathLibrary.RotateAngleAxis` _returnvalue (stale `self.ReceiveBeginPlay` _angle1) (0.0 0.0 1.0)) _returnvalue_2 NewParam))
            (:`then_1`
              (`self.CreateBullet` (`KismetMathLibrary.RotateAngleAxis` _returnvalue (stale `self.ReceiveBeginPlay` _angle2) (0.0 0.0 1.0)) _returnvalue_2 NewParam))
            (:`then_2`
              (`self.CreateBullet` (`KismetMathLibrary.RotateAngleAxis` _returnvalue (/ (stale `self.ReceiveBeginPlay` _angle1) 2.0) (0.0 0.0 1.0)) _returnvalue_2 NewParam))
            (:`then_3`
              (`self.CreateBullet` (`KismetMathLibrary.RotateAngleAxis` _returnvalue (/ (stale `self.ReceiveBeginPlay` _angle2) 2.0) (0.0 0.0 1.0)) _returnvalue_2 NewParam))
            (:`then_4`
              (goto _label))))))))

(fn `CreateBullet`
  (params (Force :type "Object.Vector Structure" :default (0.0 0.0 0.0)) (Transform :type "Object.Transform Structure") (ColorIndex :type Integer :default 0))
  (bind _machine_gun_shoot (`self.machine_gun_shoot`))
  (`|ExecutionSequence`
    (:`then_0`
      (bind _returnvalue (`|SpawnActorFromClass` "/Game/Blueprints/Weapons/MachineGunBullet.MachineGunBullet_C" (`KismetMathLibrary.MakeTransform` (.location Transform) (.rotation Transform) (.scale Transform)) true))
      (`PrimitiveComponent.AddImpulse` _returnvalue Force "None" true))
    (:`then_1`
      (`self.SetActorRotation` _returnvalue (`KismetMathLibrary.MakeRotFromZ` Force)))
    (:`then_2`
      (bind _asmaterial_instance_dynamic (cast `MaterialInstanceDynamic` (`PrimitiveComponent.GetMaterial` _returnvalue 0)))
      (bind _ascoop_game_mode (cast `/Game/Blueprints/CoopGameMode` (`GameplayStatics.GetGameMode`)))
      (bind _color (`/Game/Blueprints/ColorChangingHelpers.GetColorForIndex` ColorIndex _ascoop_game_mode))
      (`MaterialInstanceDynamic.SetVectorParameterValue` _asmaterial_instance_dynamic "Color" _color)
      (set `/Game/Blueprints/BulletProjectile.Color Index` ColorIndex _returnvalue))
    (:`then_3`
      (`GameplayStatics.PlaySoundAttached` (`AudioComponent.Sound` _machine_gun_shoot) _machine_gun_shoot "None" (0.0 0.0 0.0) "KeepRelativeOffset" false 1.0 (`GameplayStatics.GetGlobalTimeDilation`)))))

(fn `UserConstructionScript`
  (`parent.UserConstructionScript`)
  (`self.SetActorRelativeScale3D` (0.6 0.6 0.6)))