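; Weapon actor with a "Press V" pickup prompt, ammo, and experience-based levels, fired through TryShoot.
; Tick charges a fire-rate timer; TryShoot spends it and ammo in a loop, calling Shoot with a color index.
; AddExperience stops at level 2 and flags a level-up effect; GetInfoStruct packs ammo, experience and class.
; Construction applies mesh and material, compensating prompt and spring arm for root scale.
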(event EventTick
  (params (DeltaSeconds :type Float%20%28single-precision%29))
  (Utilities|FlowControl|Sequence
    (:then_0
      (if (< (Variables|Default|GetShootTimer) (Variables|Default|GetShootInterval))
        (Variables|Default|SetShootTimer (+ (Variables|Default|GetShootTimer) DeltaSeconds))))))

(fn ConstructionScript
  (bind _weaponmeshcomponent (Variables|Default|GetWeaponMeshComponent))
  (bind _pickup_text (Variables|Default|GetPickup%20Text))
  (bind _springarm1 (Variables|Default|GetSpringArm1))
  (Components|StaticMesh|SetStaticMesh _weaponmeshcomponent (Variables|Default|GetWeaponMesh))
  (Rendering|Material|SetMaterial _weaponmeshcomponent 0 (Variables|Default|GetWeaponMaterial))
  (Transformation|SetRelativeScale3D _pickup_text (* (Variables|/Script/Engine.SceneComponent|GetRelativeScale3D _pickup_text) (/ "1.000000,1.000000,1.000000" (Variables|/Script/Engine.SceneComponent|GetRelativeScale3D (VehicleSound|GetRootComponent)))))
  (Variables|/Script/Engine.SpringArmComponent|SetTargetArmLength _springarm1 (* (Variables|/Script/Engine.SpringArmComponent|GetTargetArmLength _springarm1) (/ 1.0 (.Z (Math|Vector|BreakVector (Variables|/Script/Engine.SceneComponent|GetRelativeScale3D (VehicleSound|GetRootComponent)))))))
  (Rendering|Components|TextRender|SetText (Variables|Default|GetPickup%20Text) (Utilities|String|ToString(Text) (Utilities|Text|FormatText "Press V for {name}" (Variables|Default|GetDisplayName)))))

(fn TryShoot
  (params (ColorIndex :type Integer :default 0))
  (bind _shootinterval (Variables|Default|GetShootInterval))
  (while (and (> (Variables|Default|GetAmmoCount) 0) (>= (Variables|Default|GetShootTimer) _shootinterval))
    (LocalVariables|SetShot true)
    (Utilities|FlowControl|Sequence
      (:then_0
        (Default|CallShoot ColorIndex))
      (:then_1
        (Variables|Default|SetAmmoCount (- (Variables|Default|GetAmmoCount) 1)))
      (:then_2
        (Variables|Default|SetShootTimer (- (Variables|Default|GetShootTimer) _shootinterval)))))
  (return (LocalVariables|GetShot)))

(fn GetShootLocation
  (bind _returnvalue (Transformation|GetActorTransform))
  (return (Math|Transform|TransformLocation _returnvalue (Variables|Default|GetLocalShootLocation)) (Math|Transform|TransformDirection _returnvalue (Variables|Default|GetLocalShootDirection))))

(fn GetPawn
  (bind _aspawn (Utilities|Casting|CastToPawn (Components|GetOwner (Transformation|GetAttachParent)))
    (:then
      (LocalVariables|SetPawn _aspawn))
    (:CastFailed
      _))
  (return (LocalVariables|GetPawn)))

(fn GetLevel
  (bind _experiencerequirements (Variables|Default|GetExperienceRequirements))
  (bind (_array_element _array_index) (Utilities|Array|ForEachLoopwithBreak _experiencerequirements :!label _label)
    (:LoopBody
      (if (>= (Variables|Default|GetExperience) _array_element)
        (if (== (- (Utilities|Array|Length _experiencerequirements) 1) _array_index)
          (LocalVariables|SetReturnLevel (+ _array_index 1)))
        (else
          (LocalVariables|SetReturnLevel _array_index)
          (goto _label Break))))
    (:Completed
      (return (LocalVariables|GetReturnLevel)))))

(fn SetPickupText
  (params (Visible :type Boolean))
  (bind _pickup_text (Variables|Default|GetPickup%20Text))
  (Rendering|SetVisibility _pickup_text Visible false)
  (Development|SetHiddeninGame _pickup_text (not Visible) false))

(fn AddExperience
  (params (Exp :type Integer :default 0))
  (bind _level (CallFunction|GetLevel))
  (bind _output_get (LocalVariables|SetTemporary%20level _level))
  (bind _level_2 (CallFunction|GetLevel))
  (if (!= _level_2 2)
    (Variables|Default|SetExperience (+ Exp (Variables|Default|GetExperience)))
    (bind _level_3 (CallFunction|GetLevel))
    (if (> _level_3 _output_get)
      (Variables|Default|SetNeed%20to%20play%20level%20up%20effect true)))
  (return (!= _level_2 2)))

(fn GetInfoStruct
  (return (Utilities|Struct|MakeWeaponInfoStruct (Variables|Default|GetAmmoCount) (Variables|Default|GetExperience) (.AsWeapon (Utilities|Casting|CastToWeaponClass (Utilities|GetClass self))))))