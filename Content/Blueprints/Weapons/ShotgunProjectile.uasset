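; Shotgun projectile Blueprint that deals point damage on hit and spawns a colored spark effect.
; The Hit event applies bullet damage opposite the impact impulse, then spawns sparks at the projectile's location.
; Under the co-op game mode, the sparks' particle and light colors follow the projectile's color index.
; The Bounce flag selects the spark effect variant and slightly extends Lifetime on each hit.
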(event `self.ReceiveBeginPlay`
  (`parent.ReceiveBeginPlay`))

(event `self.ReceiveActorBeginOverlap`
  (params (OtherActor :type "Actor Object Reference")))

(event `self.ReceiveTick`
  (params (DeltaSeconds :type "Float (single-precision)")))

(event `self.ReceiveHit`
  (params (MyComp :type "PrimitiveComponent Object Reference") (Other :type "Actor Object Reference") (OtherComp :type "PrimitiveComponent Object Reference") (bSelfMoved :type Boolean) (HitLocation :type "Object.Vector Structure") (HitNormal :type "Object.Vector Structure") (NormalImpulse :type "Object.Vector Structure") (Hit :type "EngineTypes.HitResult Structure (by ref)"))
  (`GameplayStatics.ApplyPointDamage` Other (`self.Damage`) (* (`KismetMathLibrary.Normal` NormalImpulse) -1.0) Hit null self "/Game/Blueprints/Weapons/BulletDamageType.BulletDamageType_C")
  (bind _returnvalue (`|SpawnActorFromClass` "/Game/Blueprints/Weapons/random_sparks_shotgun.random_sparks_shotgun_C" (`KismetMathLibrary.Conv_VectorToTransform` (`self.K2_GetActorLocation`)) true))
  (bind _ascoop_game_mode (cast `/Game/Blueprints/CoopGameMode` (`GameplayStatics.GetGameMode`)))
  (bind _color (`/Game/Blueprints/ColorChangingHelpers.GetColorForIndex` (`self.Color Index`) _ascoop_game_mode))
  (bind _effect (`/Game/Blueprints/Weapons/random_sparks_shotgun.Effect` _returnvalue))
  (`ParticleSystemComponent.SetVectorParameter` _effect "Color1" (`KismetMathLibrary.Conv_LinearColorToVector` _color))
  (bind _returnvalue_2 (`KismetMathLibrary.Conv_LinearColorToVector` _color))
  (`ParticleSystemComponent.SetVectorParameter` _effect "Color2" _returnvalue_2)
  (`LightComponent.SetLightColor` _returnvalue (`KismetMathLibrary.Conv_VectorToLinearColor` _returnvalue_2))
  (if (`self.Bounce`)
    (set `self.Lifetime` (+ (`self.Lifetime`) 0.1))
    (`/Game/Blueprints/Weapons/random_sparks_shotgun.Play effect` _returnvalue true)
    (else
      (`/Game/Blueprints/Weapons/random_sparks_shotgun.Play effect` _returnvalue false))))

(fn `UserConstructionScript`
  (`parent.UserConstructionScript`))