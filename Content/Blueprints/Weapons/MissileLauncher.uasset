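; Missile launcher weapon that fires colored missiles from its owner's shoot location when its bound Shoot event fires.
; Weapon level shapes each volley: level 0 disables homing, while level 2 doubles the missile count and zeroes their rotation.
; Each missile takes the event's color index, tinting its trail and a half-brightness body, with launch audio pitched by time dilation.
; The construction script gives the launcher a yellow material and scaled shape.
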(event `self.ReceiveBeginPlay`
  (add `self.Shoot` (delegate `OnShoot`)))

(event `OnShoot` :!signature `self.Shoot`
  (params (NewParam :type Integer))
  (bind _missilelaunchaudio (`self.MissileLaunchAudio`))
  (bind _shootatonce (`self.ShootAtOnce`))
  (bind (_world_location _world_direction) (`self.GetShootLocation`))
  (bind _owner_pawn (`self.GetPawn`))
  (bind _level (`self.GetLevel`))
  (switch `int` _level
    (:`0`
      (for _ (range 1 (+ _shootatonce 1)) :!label _label
        (`|ExecutionSequence` :!label _label_2
          (:`then_0`
            (bind _returnvalue (`|SpawnActorFromClass` "/Game/Blueprints/Weapons/Missile.Missile_C" (`KismetMathLibrary.MakeTransform` _world_location (`KismetMathLibrary.MakeRotFromZ` _world_direction)) true _owner_pawn))
            (bind _asmissile (cast `/Game/Blueprints/Weapons/Missile` _returnvalue))
            (bind _color (`/Game/Blueprints/ColorChangingHelpers.GetColorForIndex` NewParam (`GameplayStatics.GetGameMode`)))
            (set `/Game/Blueprints/Weapons/Missile.ColorIndex` NewParam _asmissile)
            (bind (_h _s _v _a) (`KismetMathLibrary.RGBToHSV` _color))
            (`MaterialInstanceDynamic.SetVectorParameterValue` (`/Game/Blueprints/Weapons/Missile.MeshMaterial` _asmissile) "Color" (`KismetMathLibrary.HSVToRGB` _h _s (* _v 0.5) _a))
            (`ParticleSystemComponent.SetVectorParameter` (`/Game/Blueprints/Weapons/Missile.Trail` _asmissile) "Color" (`KismetMathLibrary.Conv_LinearColorToVector` _color)))
          (:`then_1`
            (switch `int` _level
              (:`0`
                (set `/Game/Blueprints/Weapons/Missile.Homing` false _asmissile))
              (:`2`
                (`self.SetActorRotation` _returnvalue (struct)))))
          (:`then_2`
            (`GameplayStatics.PlaySoundAttached` (`AudioComponent.Sound` _missilelaunchaudio) _missilelaunchaudio "None" _world_location "KeepRelativeOffset" false 1.0 (`GameplayStatics.GetGlobalTimeDilation`))))))
    (:`1`
      (goto _label))
    (:`2`
      (for _ (range 1 (+ (* _shootatonce 2) 1))
        (goto _label_2)))))

(fn `UserConstructionScript`
  (`parent.UserConstructionScript`)
  (bind _returnvalue (`KismetMaterialLibrary.CreateDynamicMaterialInstance` "/Game/Materials/SimpleColor.SimpleColor"))
  (`MaterialInstanceDynamic.SetVectorParameterValue` _returnvalue "Color" (struct :`R` 1.0 :`G` 0.773006 :`A` 1.0))
  (`PrimitiveComponent.SetMaterial` 0 _returnvalue)
  (`SceneComponent.SetRelativeScale3D` (0.4 0.6 0.6)))