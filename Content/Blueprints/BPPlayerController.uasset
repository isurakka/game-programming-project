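; Player controller that moves and turns the controlled BPPlayer pawn every tick, printing a message if the cast fails.
; Movement sets physics linear velocity from normalized forward/right input scaled by Speed and DeltaSeconds.
; Yaw comes from the deprojected mouse ray's direction flattened to XY, applied as world rotation with zero pitch and roll.
; Unconnected nodes hold alternative force, transform and rotation approaches that never run.
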(event `self.ReceiveTick`
  (params (DeltaSeconds :type "Float (single-precision)"))
  (bind _asbpplayer (cast `/Game/Blueprints/BPPlayer` (`self.K2_GetPawn`))
    (:`then`
      (`|ExecutionSequence`
        (:`then_0`
          (bind _returnvalue (* (* (`KismetMathLibrary.Normal` (`KismetMathLibrary.MakeVector` (`self.GetInputAxisValue`) (`self.GetInputAxisValue`))) (`/Game/Blueprints/BPPlayer.Speed` _asbpplayer)) DeltaSeconds))
          (`PrimitiveComponent.SetPhysicsLinearVelocity` _asbpplayer _returnvalue false "None"))
        (:`then_1`
          (bind _returnvalue_2 (`KismetMathLibrary.MakeVector` (.x _returnvalue) (.y _returnvalue)))
          (`SceneComponent.K2_SetWorldRotation` _asbpplayer (`KismetMathLibrary.MakeRot` 0.0 (.yaw (`KismetMathLibrary.FindLookAtRotation` _returnvalue_2 (+ _returnvalue_2 (`KismetMathLibrary.MakeVector` (.x (`.WorldDirection` (`self.DeprojectMousePositionToWorld`))) (.y (`.WorldDirection` (`self.DeprojectMousePositionToWorld`)))))))) false))))
    (:`CastFailed`
      (`KismetSystemLibrary.PrintString` "Could not cast pawn"))))

(fn `UserConstructionScript`)