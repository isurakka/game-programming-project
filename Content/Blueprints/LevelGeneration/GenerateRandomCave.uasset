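; Procedural cave generator that spawns a grid of MazeGridCell actors and shapes it with cellular automata.
; InitializeCaveGeneration seeds random walls and smooths them in place; visited flags make only the first generation pass effective.
; A flood fill from a random open tile walls off unreached areas, regenerating if walls exceed the allowed percentage.
; It then adds three randomized unpassable border rings and colors enclosed open tiles as treasure spots.
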(event EventBeginPlay)

(fn ConstructionScript)

(fn GetTile
  (params (Row :type Integer) (Col :type Integer) (Array%20of%20Cells :type Array%20of%20Maze%20Grid%20Cell%20Object%20References))
  (bind _asmaze_grid_cell (Utilities|Casting|CastToMazeGridCell (Utilities|Array|Get(acopy) (Variables|Default|GetArray%20of%20maze%20grid%20cells) (+ (* (Variables|Default|GetGrid%20X) Row) Col)))
    (:then
      (return _asmaze_grid_cell))
    (:CastFailed
      (Development|PrintString "Getting cell failed!"))))

(fn SetTile
  (params (Value :type Maze%20Grid%20Cell%20Object%20Reference) (Row :type Integer) (Col :type Integer) (Array%20of%20Cells :type Array%20of%20Maze%20Grid%20Cell%20Object%20References)))

(fn CountAliveNeighboursOfCell
  (params (Cell%20X :type Integer) (Cell%20Y :type Integer) (2D%20Array%20of%20cells :type Array%20of%20Maze%20Grid%20Cell%20Object%20References))
  ;[1 1 1] Loop through cell's 8 neighbours with two for-loops
  (LocalVariables|SetAliveCellCount 0)
  (for _index (range -1 1)
    (for _index_2 (range -1 1)
      (LocalVariables|SetNeighbourX (+ _index Cell%20X))
      (LocalVariables|SetNeighbourY (+ _index_2 Cell%20Y))
      (if (not (and (== _index_2 0) (== _index 0)))
        (if (Math|Boolean|ORBoolean (>= (LocalVariables|GetNeighbourX) (Variables|Default|GetGrid%20X)) (< (LocalVariables|GetNeighbourX) 0) (< (LocalVariables|GetNeighbourY) 0) (>= (LocalVariables|GetNeighbourY) (Variables|Default|GetGrid%20Y)))
          (LocalVariables|SetAliveCellCount (+ (LocalVariables|GetAliveCellCount) 1))
          (else
            ;[1 1 1] Get neighbour Grid Tile instance, check whether it's dead or alive.
            (bind _tile (CallFunction|GetTile (LocalVariables|GetNeighbourX) (LocalVariables|GetNeighbourY) 2D%20Array%20of%20cells))
            (if (Variables|/Game/Blueprints/LevelGeneration/MazeGridCell.MazeGridCell_C|GetIs%20wall _tile)
              (LocalVariables|SetAliveCellCount (+ (LocalVariables|GetAliveCellCount) 1))))))))
  (return (LocalVariables|GetAliveCellCount)))

(fn SimulationStep
  (bind _array_of_maze_grid_cells (Variables|Default|GetArray%20of%20maze%20grid%20cells))
  (for _index (range 0 (- (Variables|Default|GetGrid%20X) 1))
    (Variables|Temporaryvariables|SetLoop%20X _index)
    (for _index_2 (range 0 (- (Variables|Default|GetGrid%20Y) 1))
      (Variables|Temporaryvariables|SetLoop%20Y _index_2)
      (bind _tile (CallFunction|GetTile (Variables|Temporaryvariables|GetLoop%20X) (Variables|Temporaryvariables|GetLoop%20Y) (Variables|Default|GetArray%20of%20maze%20grid%20cells)))
      (if (not (Variables|/Game/Blueprints/LevelGeneration/MazeGridCell.MazeGridCell_C|GetHas%20been%20visited _tile))
        (Variables|/Game/Blueprints/LevelGeneration/MazeGridCell.MazeGridCell_C|SetHas%20been%20visited _tile true)
        (bind _count (CallFunction|CountAliveNeighboursOfCell (Variables|Temporaryvariables|GetLoop%20X) (Variables|Temporaryvariables|GetLoop%20Y) (Variables|Default|GetArray%20of%20maze%20grid%20cells)))
        (bind _tile_2 (CallFunction|GetTile (Variables|Temporaryvariables|GetLoop%20X) (Variables|Temporaryvariables|GetLoop%20Y) (Variables|Default|GetArray%20of%20maze%20grid%20cells)))
        (if (Variables|/Game/Blueprints/LevelGeneration/MazeGridCell.MazeGridCell_C|GetIs%20wall _tile_2)
          (if (< _count (Variables|Mapgenerationadjustables|GetDeath%20limit))
            (bind _tile_3 (CallFunction|GetTile (Variables|Temporaryvariables|GetLoop%20X) (Variables|Temporaryvariables|GetLoop%20Y) _array_of_maze_grid_cells))
            (Default|SetasRegularTile _tile_3)
            (else
              (bind _tile_4 (CallFunction|GetTile (Variables|Temporaryvariables|GetLoop%20X) (Variables|Temporaryvariables|GetLoop%20Y) _array_of_maze_grid_cells))
              (Default|SetTileasWall _tile_4)))
          (elif (> _count (Variables|Mapgenerationadjustables|GetBirth%20limit))
            (bind _tile_5 (CallFunction|GetTile (Variables|Temporaryvariables|GetLoop%20X) (Variables|Temporaryvariables|GetLoop%20Y) _array_of_maze_grid_cells))
            (Default|SetTileasWall _tile_5)
            (else
              (bind _tile_6 (CallFunction|GetTile (Variables|Temporaryvariables|GetLoop%20X) (Variables|Temporaryvariables|GetLoop%20Y) _array_of_maze_grid_cells))
              (Default|SetasRegularTile _tile_6))))))))

(fn GenerateBoundWalls
  (params (Chance%20of%20tile%20becoming%20unbreakable :type Integer) (X%20Loop%20start%20index :type Integer) (X%20Loop%20end%20index :type Integer) (Y%20Loop%20Start%20Index :type Integer) (Y%20loop%20End%20Index :type Integer))
  ;[1 1 1] Top and bottom walls
  (for _index (range X%20Loop%20start%20index X%20Loop%20end%20index)
    (bind _tile (CallFunction|GetTile _index Y%20Loop%20Start%20Index (Variables|Default|GetArray%20of%20maze%20grid%20cells)))
    (if (<= (Math|Random|RandomIntegerinRange 0 100) Chance%20of%20tile%20becoming%20unbreakable)
      (Default|SetTileasUnpassable _tile)
      (bind _tile_2 (CallFunction|GetTile _index Y%20loop%20End%20Index (Variables|Default|GetArray%20of%20maze%20grid%20cells)))
      (Default|SetTileasUnpassable _tile_2)))
  ;[1 1 1] Left and right walls
  (for _index_2 (range Y%20Loop%20Start%20Index Y%20loop%20End%20Index)
    (bind _tile_3 (CallFunction|GetTile X%20Loop%20start%20index _index_2 (Variables|Default|GetArray%20of%20maze%20grid%20cells)))
    (if (<= (Math|Random|RandomIntegerinRange 0 100) Chance%20of%20tile%20becoming%20unbreakable)
      (Default|SetTileasUnpassable _tile_3)
      (bind _tile_4 (CallFunction|GetTile X%20Loop%20end%20index _index_2 (Variables|Default|GetArray%20of%20maze%20grid%20cells)))
      (Default|SetTileasUnpassable _tile_4))))

(fn PlaceTreasure
  (bind _array_of_maze_grid_cells (Variables|Default|GetArray%20of%20maze%20grid%20cells))
  (for _index (range 0 (- (Variables|Default|GetGrid%20X) 1))
    (for _index_2 (range 0 (- (Variables|Default|GetGrid%20Y) 1))
      (bind _tile (CallFunction|GetTile _index _index_2 _array_of_maze_grid_cells))
      (if (not (Variables|/Game/Blueprints/LevelGeneration/MazeGridCell.MazeGridCell_C|GetIs%20wall _tile))
        (bind _count (CallFunction|CountAliveNeighboursOfCell _index _index_2 _array_of_maze_grid_cells))
        (if (>= _count (Variables|Mapgenerationadjustables|GetPickup%20hidden%20chance))
          (Default|ChangeTileColor _tile "(R=1.000000,G=0.954856,B=0.000000,A=1.000000)"))))))

(fn GenerateLevel
  ;[1 1 1] Creater a grid of tiles that are either dead or alive, depending on the "chance for cell to span alive" variable
  (for _index (range 0 (- (Variables|Default|GetGrid%20X) 1))
    (for _index_2 (range 0 (- (Variables|Default|GetGrid%20Y) 1))
      (bind _tile (CallFunction|GetTile _index _index_2 (Variables|Default|GetArray%20of%20maze%20grid%20cells)))
      (if (<= (Math|Random|RandomInteger 100) (Variables|Default|GetChance%20for%20cell%20to%20spawn%20as%20wall))
        (Default|SetTileasWall _tile))))
  (for _index_3 (range 0 (Variables|Mapgenerationadjustables|GetAmount%20of%20generations))
    (CallFunction|SimulationStep)))

(fn FloodFill
  (bind _temporary_maze_grid_array (LocalVariables|GetTemporary%20maze%20grid%20array))
  (bind _temporary_maze_grid_array_2 (LocalVariables|GetTemporary%20maze%20grid%20array))
  (bind _returnvalue (Utilities|Array|LastIndex _temporary_maze_grid_array_2))
  (LocalVariables|SetFlood%20fill%20x (Math|Random|RandomInteger (Variables|Default|GetGrid%20X)) :!label _label)
  (LocalVariables|SetFlood%20fill%20y (Math|Random|RandomInteger (Variables|Default|GetGrid%20Y)))
  (bind _tile (CallFunction|GetTile (LocalVariables|GetFlood%20fill%20x) (LocalVariables|GetFlood%20fill%20y) (Variables|Default|GetArray%20of%20maze%20grid%20cells)))
  (if (Variables|/Game/Blueprints/LevelGeneration/MazeGridCell.MazeGridCell_C|GetIs%20wall _tile)
    (goto _label)
    (else
      (Utilities|Array|Add _temporary_maze_grid_array _tile)
      (while (> (Utilities|Array|Length _temporary_maze_grid_array) 0)
        (LocalVariables|SetTemporary%20maze%20cell (Utilities|Array|Get(acopy) _temporary_maze_grid_array_2 _returnvalue))
        (Utilities|Array|RemoveIndex (LocalVariables|GetTemporary%20maze%20grid%20array) _returnvalue)
        (if (not (Variables|/Game/Blueprints/LevelGeneration/MazeGridCell.MazeGridCell_C|GetIs%20wall (LocalVariables|GetTemporary%20maze%20cell)))
          (bind (_x _y) (CallFunction|GetCoordinatesfromTile (LocalVariables|GetTemporary%20maze%20cell)))
          (LocalVariables|SetFlood%20fill%20x _x)
          (LocalVariables|SetFlood%20fill%20y _y)
          (Default|ChangeTileColor (LocalVariables|GetTemporary%20maze%20cell) "(R=0.780744,G=0.019184,B=1.000000,A=1.000000)")
          (Variables|/Game/Blueprints/LevelGeneration/MazeGridCell.MazeGridCell_C|SetHas%20been%20visited (LocalVariables|GetTemporary%20maze%20cell) true)
          (if (>= (+ (LocalVariables|GetFlood%20fill%20x) 1) (Variables|Default|GetGrid%20X))
            _
            (else
              (bind _tile_2 (CallFunction|GetTile (+ (LocalVariables|GetFlood%20fill%20x) 1) (LocalVariables|GetFlood%20fill%20y) (Variables|Default|GetArray%20of%20maze%20grid%20cells)))
              (if (Variables|/Game/Blueprints/LevelGeneration/MazeGridCell.MazeGridCell_C|GetHas%20been%20visited _tile_2)
                _
                (else
                  (Utilities|Array|Add (LocalVariables|GetTemporary%20maze%20grid%20array) _tile_2)))))
          (if (>= (+ (LocalVariables|GetFlood%20fill%20y) 1) (Variables|Default|GetGrid%20Y))
            _
            (else
              (bind _tile_3 (CallFunction|GetTile (LocalVariables|GetFlood%20fill%20x) (+ (LocalVariables|GetFlood%20fill%20y) 1) (Variables|Default|GetArray%20of%20maze%20grid%20cells)))
              (if (Variables|/Game/Blueprints/LevelGeneration/MazeGridCell.MazeGridCell_C|GetHas%20been%20visited _tile_3)
                _
                (else
                  (Utilities|Array|Add (LocalVariables|GetTemporary%20maze%20grid%20array) _tile_3)))))
          (if (== (- (LocalVariables|GetFlood%20fill%20x) 1) -1)
            (if (not (== (- (LocalVariables|GetFlood%20fill%20y) 1) 0))
              (bind _tile_4 (CallFunction|GetTile (LocalVariables|GetFlood%20fill%20x) (- (LocalVariables|GetFlood%20fill%20y) 1) (Variables|Default|GetArray%20of%20maze%20grid%20cells) :!label _label_2))
              (if (not (Variables|/Game/Blueprints/LevelGeneration/MazeGridCell.MazeGridCell_C|GetHas%20been%20visited _tile_4))
                (Utilities|Array|Add (LocalVariables|GetTemporary%20maze%20grid%20array) _tile_4)))
            (else
              (bind _tile_5 (CallFunction|GetTile (- (LocalVariables|GetFlood%20fill%20x) 1) (LocalVariables|GetFlood%20fill%20y) (Variables|Default|GetArray%20of%20maze%20grid%20cells)))
              (if (Variables|/Game/Blueprints/LevelGeneration/MazeGridCell.MazeGridCell_C|GetHas%20been%20visited _tile_5)
                (goto _label_2)
                (else
                  (Utilities|Array|Add (LocalVariables|GetTemporary%20maze%20grid%20array) _tile_5)
                  (goto _label_2))))))))))

(fn GetCoordinatesfromTile
  (params (Cell :type Maze%20Grid%20Cell%20Object%20Reference))
  (bind _array_of_maze_grid_cells (Variables|Default|GetArray%20of%20maze%20grid%20cells))
  (bind _returnvalue (Utilities|Array|FindItem _array_of_maze_grid_cells Cell))
  (bind _item (Utilities|Array|Get(acopy) _array_of_maze_grid_cells _returnvalue))
  (return (Variables|/Game/Blueprints/LevelGeneration/MazeGridCell.MazeGridCell_C|GetX%20position _item) (Variables|/Game/Blueprints/LevelGeneration/MazeGridCell.MazeGridCell_C|GetY%20position _item)))

(fn InitializeCaveGeneration
  (bind _array_of_maze_grid_cells (Variables|Default|GetArray%20of%20maze%20grid%20cells))
  (Variables|Default|SetGrid%20X 50)
  (Variables|Default|SetGrid%20Y 50)
  (Variables|Mapgenerationadjustables|SetPickup%20hidden%20chance 6)
  (Variables|Default|SetMesh%20width 400)
  (Variables|Mapgenerationadjustables|SetBirth%20limit 4)
  (Variables|Mapgenerationadjustables|SetDeath%20limit 3)
  (Variables|Default|SetChance%20for%20cell%20to%20spawn%20as%20wall 40)
  (Variables|Mapgenerationadjustables|SetAmount%20of%20generations 4)
  (Variables|Default|SetAcceptable%20percentage%20of%20wall%20tiles 60)
  ;[1 1 1] Creater a grid of tiles that are either dead or alive, depending on the "chance for cell to span alive" variable
  (for _index (range 0 (- (Variables|Default|GetGrid%20X) 1))
    (for _index_2 (range 0 (- (Variables|Default|GetGrid%20Y) 1))
      (bind _returnvalue (Game|SpawnActorfromClass "/Game/Blueprints/LevelGeneration/MazeGridCell.MazeGridCell_C" (Math|Conversions|ToTransform(Vector) (Math|Vector|MakeVector (Math|Conversions|ToFloat(Integer) (* _index (Variables|Default|GetMesh%20width))) (Math|Conversions|ToFloat(Integer) (* _index_2 (Variables|Default|GetMesh%20width))) 0.0)) false 0))
      (Variables|/Game/Blueprints/LevelGeneration/MazeGridCell.MazeGridCell_C|SetX%20position _returnvalue _index)
      (Variables|/Game/Blueprints/LevelGeneration/MazeGridCell.MazeGridCell_C|SetY%20position _returnvalue _index_2)
      (Utilities|Array|Add (Variables|Default|GetArray%20of%20maze%20grid%20cells) _returnvalue)))
  (CallFunction|GenerateLevel :!label _label)
  (for _array_element (Variables|Default|GetArray%20of%20maze%20grid%20cells)
    (Variables|/Game/Blueprints/LevelGeneration/MazeGridCell.MazeGridCell_C|SetHas%20been%20visited _array_element false))
  (CallFunction|FloodFill)
  (Variables|Default|SetAmount%20of%20wall%20tiles 0)
  (for _array_element_2 _array_of_maze_grid_cells
    (if (not (Variables|/Game/Blueprints/LevelGeneration/MazeGridCell.MazeGridCell_C|GetHas%20been%20visited _array_element_2))
      (Default|SetTileasWall _array_element_2)))
  (for _array_element_3 _array_of_maze_grid_cells
    (if (Variables|/Game/Blueprints/LevelGeneration/MazeGridCell.MazeGridCell_C|GetIs%20wall _array_element_3)
      (Variables|Default|SetAmount%20of%20wall%20tiles (+ (Variables|Default|GetAmount%20of%20wall%20tiles) 1))))
  (if (> (Math|Float|Floor (* (/ (Math|Conversions|ToFloat(Integer) (Variables|Default|GetAmount%20of%20wall%20tiles)) (Math|Conversions|ToFloat(Integer) (* (Variables|Default|GetGrid%20Y) (Variables|Default|GetGrid%20X)))) 1e+02)) (Variables|Default|GetAcceptable%20percentage%20of%20wall%20tiles))
    (Development|PrintString "regenerating map")
    (CallFunction|ResetTiles)
    (goto _label)
    (else
      (CallFunction|GenerateBoundWalls 100 0 (- (Variables|Default|GetGrid%20X) 1) 0 (- (Variables|Default|GetGrid%20Y) 1))
      (CallFunction|GenerateBoundWalls 70 1 (- (Variables|Default|GetGrid%20X) 2) 1 (- (Variables|Default|GetGrid%20Y) 2))
      (CallFunction|GenerateBoundWalls 60 2 (- (Variables|Default|GetGrid%20X) 3) 2 (- (Variables|Default|GetGrid%20Y) 3))
      (CallFunction|PlaceTreasure)
      (for _array_element_4 (Variables|Default|GetArray%20of%20maze%20grid%20cells)
        (Default|RemoveWall _array_element_4)))))

(fn ResetTiles
  (for _array_element (Variables|Default|GetArray%20of%20maze%20grid%20cells)
    (Variables|/Game/Blueprints/LevelGeneration/MazeGridCell.MazeGridCell_C|SetIs%20wall _array_element false)
    (Variables|/Game/Blueprints/LevelGeneration/MazeGridCell.MazeGridCell_C|SetHas%20been%20visited _array_element false)))