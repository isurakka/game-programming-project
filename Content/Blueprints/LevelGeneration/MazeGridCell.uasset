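; Maze grid cell actor for level generation, with a floor tile and a wall component.
; A dynamic material created in the construction script lets each state change recolor the floor.
; State functions set IsWall and IsUnpassable to mark unpassable, wall or regular tiles; setting a tile passable turns it into an ordinary wall.
; RemoveWall destroys the wall component on cells not flagged as walls.
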(fn `ChangeTileColor`
  (params (Color :type "Object.LinearColor Structure"))
  (`MaterialInstanceDynamic.SetVectorParameterValue` (`self.TileMaterial`) "Color" Color))

(fn `Remove wall`
  (if (not (`self.Is wall`))
    (`ActorComponent.K2_DestroyComponent` (`self.Wall`))))

(fn `Set as regular tile`
  (set `self.Is wall` false)
  (set `self.Is unpassable` false)
  (`self.ChangeTileColor` (struct :`R` 0.56 :`G` 0.43435 :`B` 0.178542 :`A` 1.0)))

(fn `Set Tile as Passable`
  (set `self.Is unpassable` false)
  (`self.Set Tile As Wall`))

(fn `Set Tile As Unpassable`
  (`self.ChangeTileColor` (struct :`G` 1.0 :`B` 0.115803 :`A` 1.0))
  (set `self.Is unpassable` true)
  (set `self.Is wall` true))

(fn `Set Tile As Wall`
  (`self.ChangeTileColor` (struct :`R` 0.305 :`G` 0.152061 :`A` 1.0))
  (set `self.Is wall` true))

(fn `UserConstructionScript`
  (bind _returnvalue (`PrimitiveComponent.CreateDynamicMaterialInstance` (`self.FloorTile`) 0 null))
  (set `self.TileMaterial` _returnvalue))