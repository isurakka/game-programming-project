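; GlowingMushroom is a level-generation prop that gives each mushroom a random look when play begins.
; It picks a color from ColorChoices and applies it to both the glow light and a dynamic material instance on the cap.
; It also randomly chooses one of two low-poly cap meshes and sets a random yaw and roll on the actor, keeping pitch at zero.
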(event `self.ReceiveBeginPlay`
  (bind _low_poly_mushroom_02_cap (`self.Low_Poly_Mushroom_02_Cap`))
  (bind _returnvalue (`KismetMaterialLibrary.CreateDynamicMaterialInstance` "/Game/Blueprints/LevelGeneration/MushroomMaterial.MushroomMaterial"))
  (set `self.ShroomCapColor` (`KismetArrayLibrary.Array_Get` (`self.ColorChoices`) (`KismetMathLibrary.RandomIntegerInRange` 0 (- (`KismetArrayLibrary.Array_Length` (`self.ColorChoices`)) 1))))
  (`LightComponent.SetLightColor` (`self.ShroomGlow`) (`self.ShroomCapColor`))
  (`MaterialInstanceDynamic.SetVectorParameterValue` _returnvalue "Color" (`self.ShroomCapColor`))
  (if (`KismetMathLibrary.RandomBool`)
    (`StaticMeshComponent.SetStaticMesh` _low_poly_mushroom_02_cap "/Game/Blueprints/Props/Misc/Mushrooms/Low_Poly_Mushroom_01_Cap.Low_Poly_Mushroom_01_Cap")
    (else
      (`StaticMeshComponent.SetStaticMesh` _low_poly_mushroom_02_cap "/Game/Blueprints/Props/Misc/Mushrooms/Low_Poly_Mushroom_02_Cap.Low_Poly_Mushroom_02_Cap")))
  (`PrimitiveComponent.SetMaterial` (`self.Low_Poly_Mushroom_02_Cap`) 0 _returnvalue)
  (`self.SetActorRotation` (`KismetMathLibrary.MakeRot` 0.0 (.yaw (`KismetMathLibrary.RandomRotator` false)) (.roll (`KismetMathLibrary.RandomRotator` false)))))

(event `self.ReceiveActorBeginOverlap`
  (params (OtherActor :type "Actor Object Reference")))

(event `self.ReceiveTick`
  (params (DeltaSeconds :type "Float (single-precision)")))

(fn `UserConstructionScript`)