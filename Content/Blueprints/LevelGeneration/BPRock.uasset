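; BPRock is a level-generation rock actor that randomizes its look for visual variety.
; The construction script picks a random mesh, yaw and non-uniform scale within ScaleRange, then swaps material slot 0 for a dynamic instance.
; On BeginPlay, it sets that instance's Color parameter to a random entry from PossibleColors.
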(event `self.ReceiveBeginPlay`
  (bind _possible_colors (`self.Possible Colors`))
  (bind _asmaterial_instance_dynamic (cast `MaterialInstanceDynamic` (`PrimitiveComponent.GetMaterial` (`self.Mesh`) 0)))
  (`MaterialInstanceDynamic.SetVectorParameterValue` _asmaterial_instance_dynamic "Color" (`KismetArrayLibrary.Array_Get` _possible_colors (`KismetMathLibrary.RandomIntegerInRange` 0 (`KismetArrayLibrary.Array_LastIndex` _possible_colors)))))

(event `self.ReceiveActorBeginOverlap`
  (params (OtherActor :type "Actor Object Reference")))

(event `self.ReceiveTick`
  (params (DeltaSeconds :type "Float (single-precision)")))

(fn `UserConstructionScript`
  (bind _mesh (`self.Mesh`))
  (bind _array_of_meshes (`self.Array of meshes`))
  (bind (_x _y) (`KismetMathLibrary.BreakVector2D` (`self.ScaleRange`)))
  (`StaticMeshComponent.SetStaticMesh` (`self.Mesh`) (`KismetArrayLibrary.Array_Get` _array_of_meshes (`KismetMathLibrary.RandomIntegerInRange` 0 (`KismetArrayLibrary.Array_LastIndex` _array_of_meshes))))
  (`self.SetActorRotation` (`KismetMathLibrary.MakeRot` 0.0 (`KismetMathLibrary.RandomFloatInRange` 0.0 360.0)))
  (`SceneComponent.SetWorldScale3D` (`self.Mesh`) (`KismetMathLibrary.MakeVector` (`KismetMathLibrary.RandomFloatInRange` _x _y) (`KismetMathLibrary.RandomFloatInRange` _x _y) (`KismetMathLibrary.RandomFloatInRange` _x _y)))
  (bind _returnvalue (`KismetMaterialLibrary.CreateDynamicMaterialInstance` (`PrimitiveComponent.GetMaterial` _mesh 0)))
  (`PrimitiveComponent.SetMaterial` _mesh 0 _returnvalue))