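; Destructible crate prop that swaps itself for a fractured stand-in and passes on its drop settings when its HealthComponent reports death.
; OnDie disables and hides the crate, spawns an InstantlyDestructibleCrate at its transform and copies linear and angular velocity to it.
; It forwards ActorToSpawnOnDestruction and an Amount scaled by co-op player count, then applies huge damage to shatter the replacement.
; The construction script fixes a uniform reduced scale.
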(event `self.ReceiveBeginPlay`)

(event `self.ReceiveActorBeginOverlap`
  (params (OtherActor :type "Actor Object Reference")))

(event `self.ReceiveTick`
  (params (DeltaSeconds :type "Float (single-precision)")))

(event `self.HealthComponent.OnDie`
  (bind _returnvalue (`KismetMathLibrary.RandomUnitVector`))
  (bind _crate (`self.Crate`))
  (`PrimitiveComponent.SetSimulatePhysics` _crate false)
  (`PrimitiveComponent.SetCollisionEnabled` _crate "NoCollision")
  (`SceneComponent.SetVisibility` false)
  (bind _returnvalue_2 (`|SpawnActorFromClass` "/Game/Blueprints/Props/InstantlyDestructibleCrate.InstantlyDestructibleCrate_C" (`self.GetTransform`) true))
  (`|ExecutionSequence`
    (:`then_0`
      (bind _returnvalue_3 (`PrimitiveComponent.GetPhysicsAngularVelocity` "None"))
      (`PrimitiveComponent.SetPhysicsAngularVelocity` _returnvalue_2 _returnvalue_3 false "None"))
    (:`then_1`
      (bind _returnvalue_4 (`PrimitiveComponent.GetPhysicsLinearVelocity` "None"))
      (`PrimitiveComponent.SetAllPhysicsLinearVelocity` _returnvalue_2 _returnvalue_4 false))
    (:`then_2`
      (`|ExecutionSequence`
        (:`then_0`
          (set `/Game/Blueprints/Props/InstantlyDestructibleCrate.ActorToSpawnOnDestruction` (`self.ActorToSpawnOnDestruction`) _returnvalue_2))
        (:`then_1`
          (bind _ascoop_game_mode (cast `/Game/Blueprints/CoopGameMode` (`GameplayStatics.GetGameMode`)))
          (set `/Game/Blueprints/Props/InstantlyDestructibleCrate.Amount` (`KismetMathLibrary.FCeil` (* (`self.Amount`) (* (`/Game/Blueprints/CoopGameMode.Number of players` _ascoop_game_mode) (`self.PlayerCountMultiplier`)))) _returnvalue_2))
        (:`then_2`
          (`DestructibleComponent.ApplyDamage` _returnvalue_2 100000.0 _returnvalue _returnvalue 10.0 :!label _label))
        (:`then_10`
          (goto _label))))))

(fn `UserConstructionScript`
  (`SceneComponent.SetWorldScale3D` (0.6 0.6 0.6)))