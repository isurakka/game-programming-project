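; Torch prop with a point light, fire effect and looping sound, which can be switched off through Deactivate.
; Tick matches the audio pitch to global time dilation so the sound follows slow or fast motion.
; CheckForCollision destroys the torch if a small sphere at its location overlaps world static or dynamic objects, and returns whether it was clear.
; Logic for randomly starting unlit exists but is disconnected.
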(event `self.ReceiveBeginPlay`)

(event `self.ReceiveActorBeginOverlap`
  (params (OtherActor :type "Actor Object Reference")))

(event `self.ReceiveTick`
  (params (DeltaSeconds :type "Float (single-precision)"))
  (`AudioComponent.SetPitchMultiplier` (`self.Audio`) (`GameplayStatics.GetGlobalTimeDilation`)))

(fn `Check for collision`
  (returns (`Was spawn succesful` :type Boolean))
  (bind (_outactors _returnvalue) (`KismetSystemLibrary.SphereOverlapActors_NEW` (`self.K2_GetActorLocation`) 5.0 (`|MakeArray` "ObjectTypeQuery1" "ObjectTypeQuery2" :!type "EngineTypes.EObjectTypeQuery Enum")))
  (if _returnvalue
    (`self.K2_DestroyActor`))
  (return (not _returnvalue)))

(fn `Deactivate`
  (`SceneComponent.SetVisibility` (`self.PointLight`) false false)
  (`AudioComponent.Stop` (`self.Audio`))
  (`SceneComponent.SetVisibility` (`self.Torch fire`) false false))

(fn `UserConstructionScript`)