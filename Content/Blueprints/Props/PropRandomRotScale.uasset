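; A prop actor that varies its placed appearance through random rotation and scale.
; Its construction script assigns the configurable static mesh, then sets the actor to a random yaw with zero pitch and roll.
; Each mesh axis gets its own random scale within ScaleRange, so scaling is non-uniform and rerolls whenever construction reruns.
; The event graph holds only disabled default events.
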(event `self.ReceiveBeginPlay`)

(event `self.ReceiveActorBeginOverlap`
  (params (OtherActor :type "Actor Object Reference")))

(event `self.ReceiveTick`
  (params (DeltaSeconds :type "Float (single-precision)")))

(fn `UserConstructionScript`
  (bind (_x _y) (`KismetMathLibrary.BreakVector2D` (`self.ScaleRange`)))
  (`StaticMeshComponent.SetStaticMesh` (`self.Mesh`) (`self.StaticMesh`))
  (`self.SetActorRotation` (`KismetMathLibrary.MakeRot` 0.0 (`KismetMathLibrary.RandomFloatInRange` 0.0 360.0)))
  (`SceneComponent.SetWorldScale3D` (`self.Mesh`) (`KismetMathLibrary.MakeVector` (`KismetMathLibrary.RandomFloatInRange` _x _y) (`KismetMathLibrary.RandomFloatInRange` _x _y) (`KismetMathLibrary.RandomFloatInRange` _x _y))))