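; AmmoDestructibleCrate is a breakable crate prop that spills ammo when its destructible mesh fractures.
; On fracture, it casts the game mode to CoopGameMode and repeatedly calls its CreateAmmo to obtain several ammo actors.
; Each is moved to a random point within the crate's bounds, taking the crate's rotation and keeping its own scale.
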(event `self.ReceiveBeginPlay`)

(event `self.ReceiveActorBeginOverlap`
  (params (OtherActor :type "Actor Object Reference")))

(event `self.ReceiveTick`
  (params (DeltaSeconds :type "Float (single-precision)")))

(event `self.DestructibleMesh.OnComponentFracture`
  (params (HitPoint :type "Object.Vector Structure (by ref)") (HitDirection :type "Object.Vector Structure (by ref)"))
  (bind (_origin _boxextent) (`self.GetActorBounds` false))
  (bind _ascoop_game_mode (cast `/Game/Blueprints/CoopGameMode` (`GameplayStatics.GetGameMode`)))
  (for _ (range 6)
    (bind _instance (`/Game/Blueprints/CoopGameMode.CreateAmmo` _ascoop_game_mode))
    (`self.K2_SetActorTransform` _instance (`KismetMathLibrary.MakeTransform` (`KismetMathLibrary.RandomPointInBoundingBox` _origin _boxextent) (.rotation (`SceneComponent.K2_GetComponentToWorld`)) (.scale (`self.GetTransform` _instance))) false)))

(fn `UserConstructionScript`)