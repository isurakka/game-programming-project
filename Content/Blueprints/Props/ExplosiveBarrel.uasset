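; An explosive barrel prop that blows up and deals area damage when its HealthComponent reports death.
; OnDie calls Explode, which spawns the explosion effect, hides the barrel and applies radial damage with falloff, using its own damage type.
; Explode neither destroys the actor nor passes an instigator.
; An older inline health and delayed-explosion chain remains in the event graph, disconnected, and AnyDamage does nothing.
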(event `self.ReceiveAnyDamage`
  (params (Damage :type "Float (single-precision)") (DamageType :type "DamageType Object Reference") (InstigatedBy :type "Controller Object Reference") (DamageCauser :type "Actor Object Reference")))

(event `self.HealthComponent.OnDie`
  (`self.Explode`))

(fn `Explode`
  (bind _returnvalue (`SceneComponent.K2_GetComponentToWorld`))
  (`|SpawnActorFromClass` "/Game/Blueprints/Blueprint_Effect_Explosion.Blueprint_Effect_Explosion_C" _returnvalue true)
  (set `self.ExplosionLocation` (.location _returnvalue))
  (`self.SetActorHiddenInGame` true)
  (`GameplayStatics.ApplyRadialDamageWithFalloff` :`BaseDamage` (`self.ExplosionDamage`) :`Origin` (`self.ExplosionLocation`) :`DamageOuterRadius` (`self.ExplosionRadius`) :`DamageFalloff` 1.0 :`DamageTypeClass` "/Game/Blueprints/Props/ExplosiveBarrelDamage.ExplosiveBarrelDamage_C" :`DamageCauser` self))

(fn `UserConstructionScript`)