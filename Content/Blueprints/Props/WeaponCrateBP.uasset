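; Weapon crate prop that can be destroyed, swapping itself for a destructible version when it dies.
; On the health component's death event, it disables the crate's physics and collision, hides it, and spawns the configured destructible at its transform.
; It then immediately applies heavy damage with a random impulse direction to that spawn so it breaks apart.
; The construction script sets a uniform reduced scale.
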(event `self.ReceiveBeginPlay`)

(event `self.ReceiveActorBeginOverlap`
  (params (OtherActor :type "Actor Object Reference")))

(event `self.ReceiveTick`
  (params (DeltaSeconds :type "Float (single-precision)")))

(event `self.HealthComponent.OnDie`
  (bind _returnvalue (`KismetMathLibrary.RandomUnitVector`))
  (bind _crate (`self.Crate`))
  (`PrimitiveComponent.SetSimulatePhysics` _crate false)
  (`PrimitiveComponent.SetCollisionEnabled` _crate "NoCollision")
  (`SceneComponent.SetVisibility` false)
  (bind _returnvalue_2 (`|SpawnActorFromClass` (`self.DestructibleToSpawn`) (`self.GetTransform`)))
  (`DestructibleComponent.ApplyDamage` _returnvalue_2 1000.0 _returnvalue _returnvalue 10.0))

(fn `UserConstructionScript`
  (`SceneComponent.SetWorldScale3D` (0.6 0.6 0.6)))