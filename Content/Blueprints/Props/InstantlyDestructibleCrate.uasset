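; A destructible crate prop that spawns loot or other configurable actors when its mesh fractures.
; On the fracture event it spawns Amount copies of ActorToSpawnOnDestruction at random points within its bounds, using its own rotation and scale.
; Each spawned actor's mesh components inherit the crate's linear and angular physics velocity, carrying its motion through the break.
; The spawn loop also gives the crate a short lifespan so it removes itself afterwards.
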(event `self.ReceiveBeginPlay`)

(event `self.ReceiveActorBeginOverlap`
  (params (OtherActor :type "Actor Object Reference")))

(event `self.ReceiveTick`
  (params (DeltaSeconds :type "Float (single-precision)")))

(event `self.DestructibleMesh.OnComponentFracture`
  (params (HitPoint :type "Object.Vector Structure (by ref)") (HitDirection :type "Object.Vector Structure (by ref)"))
  (bind (_origin _boxextent) (`self.GetActorBounds` false))
  (for _ (range (`self.Amount`))
    (bind _returnvalue (`|SpawnActorFromClass` (`self.ActorToSpawnOnDestruction`) (`KismetMathLibrary.MakeTransform` (`KismetMathLibrary.RandomPointInBoundingBox` _origin _boxextent) (.rotation (`SceneComponent.K2_GetComponentToWorld`)) (.scale (`self.GetTransform`))) true))
    (bind _returnvalue_2 (`PrimitiveComponent.GetPhysicsAngularVelocity` "None"))
    (bind _returnvalue_3 (`PrimitiveComponent.GetPhysicsLinearVelocity` "None"))
    (for _array_element (`self.K2_GetComponentsByClass` _returnvalue "/Script/Engine.MeshComponent")
      (`|ExecutionSequence`
        (:`then_0`
          (`PrimitiveComponent.SetPhysicsAngularVelocity` _array_element _returnvalue_2 false "None"))
        (:`then_1`
          (`PrimitiveComponent.SetPhysicsLinearVelocity` _array_element _returnvalue_3 false "None"))))
    (`self.SetLifeSpan` 3.0)))

(fn `UserConstructionScript`)