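; EnemySpawnBounds is a spawn Blueprint that creates AI enemies and reports its enemy count to the co-op game mode.
; One second after BeginPlay, it casts to CoopGameMode and adds the result of CalculateSpawnCount to the total number of enemies.
; SpawnOne spawns the configured pawn class at a given transform, keeping only yaw, ignoring collision failure and always returning false.
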(event `self.ReceiveBeginPlay`
  (`KismetSystemLibrary.Delay` 1.0)
  (bind _ascoop_game_mode (cast `/Game/Blueprints/CoopGameMode` (`GameplayStatics.GetGameMode`)))
  (bind _count (`self.CalculateSpawnCount`))
  (`/Game/Blueprints/CoopGameMode.Increment total number of enemies` _ascoop_game_mode _count))

(event `self.ReceiveActorBeginOverlap`
  (params (OtherActor :type "Actor Object Reference"))
  (`parent.ReceiveActorBeginOverlap` null))

(event `self.ReceiveTick`
  (params (DeltaSeconds :type "Float (single-precision)")))

(fn `SpawnOne`
  (params (Transform :type "Object.Transform Structure"))
  (returns (Potato :type Boolean))
  (`AIBlueprintHelperLibrary.SpawnAIFromClass` (`self.Class`) null (.location Transform) (`KismetMathLibrary.MakeRot` 0.0 (.yaw (.rotation Transform))) true)
  (return false))

(fn `UserConstructionScript`
  (`parent.UserConstructionScript`))