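; Helper functions for color changing that read the Colors array on the CoopGameMode.
; GetNextColorIndex advances an index and wraps to zero at the end of the array, while GetColorForIndex returns the color at a given index.
; Both take a game mode and pass it through a shared CastGameMode helper, which prints an error string if the cast fails.
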(fn GetNextColorIndex
  (params (CurrentIndex :type Integer) (GameMode :type Game%20Mode%20Object%20Reference))
  (bind _returnvalue (+ CurrentIndex 1))
  (bind _gamemode (CallFunction|CastGameMode GameMode))
  (LocalVariables|SetReturnIndex _returnvalue)
  (if (>= _returnvalue (Utilities|Array|Length (Variables|/Game/Blueprints/CoopGameMode.CoopGameMode_C|GetColors _gamemode)))
    (LocalVariables|SetReturnIndex 0))
  (return (LocalVariables|GetReturnIndex)))

(fn CastGameMode
  (params (ToBeCasted :type Game%20Mode%20Object%20Reference))
  (bind _ascoop_game_mode (Utilities|Casting|CastToCoopGameMode ToBeCasted)
    (:then
      (return _ascoop_game_mode))
    (:CastFailed
      (Development|PrintString ToBeCasted "COULD NOT CAST GAMEMODE IN COLOR CHANGING HELPER!"))))

(fn GetColorforIndex
  (params (Index :type Integer) (GameMode :type Game%20Mode%20Object%20Reference))
  (bind _gamemode (CallFunction|CastGameMode GameMode))
  (return (Utilities|Array|Get(acopy) (Variables|/Game/Blueprints/CoopGameMode.CoopGameMode_C|GetColors _gamemode) Index)))