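; BulletProjectile is a bullet actor that deals point damage to whatever it hits and then destroys itself.
; On hit, it applies Damage with BulletDamageType, using the negated impact impulse as direction, and destroys itself after a very brief delay.
; An unobstructed bullet expires after Lifetime.
; The construction script gives it a dynamic material instance and applies a relative rotation.
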(event `self.ReceiveBeginPlay`
  (`KismetSystemLibrary.Delay` (`self.Lifetime`))
  (`self.K2_DestroyActor`))

(event `self.ReceiveActorBeginOverlap`
  (params (OtherActor :type "Actor Object Reference")))

(event `self.ReceiveTick`
  (params (DeltaSeconds :type "Float (single-precision)")))

(event `self.ReceiveHit`
  (params (MyComp :type "PrimitiveComponent Object Reference") (Other :type "Actor Object Reference") (OtherComp :type "PrimitiveComponent Object Reference") (bSelfMoved :type Boolean) (HitLocation :type "Object.Vector Structure") (HitNormal :type "Object.Vector Structure") (NormalImpulse :type "Object.Vector Structure") (Hit :type "EngineTypes.HitResult Structure (by ref)"))
  (`GameplayStatics.ApplyPointDamage` Other (`self.Damage`) (* (`KismetMathLibrary.Normal` NormalImpulse) -1.0) Hit null self "/Game/Blueprints/Weapons/BulletDamageType.BulletDamageType_C")
  (`KismetSystemLibrary.Delay` 0.001)
  (`self.K2_DestroyActor`))

(fn `UserConstructionScript`
  (bind _returnvalue (`KismetMaterialLibrary.CreateDynamicMaterialInstance` (`PrimitiveComponent.GetMaterial` 0)))
  (`PrimitiveComponent.SetMaterial` 0 _returnvalue)
  (`self.K2_SetActorRelativeRotation` (`self.Relative rotation`)))