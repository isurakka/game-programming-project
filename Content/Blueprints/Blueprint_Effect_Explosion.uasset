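; Explosion effect Blueprint that pairs a particle effect with a randomly chosen explosion sound.
; The construction script picks a random blast color from a unit vector and plays a random sound from the SFX array, pitched by global time dilation.
; Activate passes the blast color to the particle system as a vector parameter and starts it.
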(fn `Activate`
  (bind _p_explosion (`self.P_Explosion`))
  (`ParticleSystemComponent.SetVectorParameter` _p_explosion "BlastColor" (`KismetMathLibrary.Conv_LinearColorToVector` (`self.Blast color`)))
  (`ActorComponent.Activate` _p_explosion false))

(fn `UserConstructionScript`
  (bind _explosion_sfx (`self.Explosion SFX`))
  (bind _explosion_audio (`self.Explosion Audio`))
  (set `self.Blast color` (`KismetMathLibrary.Conv_VectorToLinearColor` (`KismetMathLibrary.RandomUnitVector`)))
  (`AudioComponent.SetSound` _explosion_audio (`KismetArrayLibrary.Array_Get` _explosion_sfx (`KismetMathLibrary.RandomIntegerInRange` 0 (- (`KismetArrayLibrary.Array_Length` _explosion_sfx) 1))))
  (`AudioComponent.SetPitchMultiplier` _explosion_audio (`GameplayStatics.GetGlobalTimeDilation`))
  (`AudioComponent.Play` _explosion_audio 0.0))