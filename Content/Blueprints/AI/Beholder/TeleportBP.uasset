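; TeleportBP is an actor in the Beholder AI folder that spawns a group of swarm enemies around itself; despite its name, it contains no teleport logic.
; One second after BeginPlay, it calls SpawnSwarmEnemy, which creates four SwarmEnemy actors at equal offsets on either side along the world X and Y axes.
; Each spawned enemy receives its default controller immediately.
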(event `self.ReceiveBeginPlay`
  (`KismetSystemLibrary.Delay` 1.0)
  (`self.Spawn swarm enemy`))

(event `self.ReceiveActorBeginOverlap`
  (params (OtherActor :type "Actor Object Reference")))

(event `self.ReceiveTick`
  (params (DeltaSeconds :type "Float (single-precision)")))

(fn `Spawn swarm enemy`
  (bind _x (.x (`self.K2_GetActorLocation`)))
  (bind _y (.y (`self.K2_GetActorLocation`)))
  (bind _z (.z (`self.K2_GetActorLocation`)))
  (`|ExecutionSequence`
    (:`then_0`
      (bind _returnvalue (`|SpawnActorFromClass` "/Game/Blueprints/AI/Swarm_Enemy/SwarmEnemy.SwarmEnemy_C" (`KismetMathLibrary.Conv_VectorToTransform` (`KismetMathLibrary.MakeVector` (+ _x 100.0) _y _z))))
      (`Pawn.SpawnDefaultController` _returnvalue))
    (:`then_1`
      (bind _returnvalue_2 (`|SpawnActorFromClass` "/Game/Blueprints/AI/Swarm_Enemy/SwarmEnemy.SwarmEnemy_C" (`KismetMathLibrary.Conv_VectorToTransform` (`KismetMathLibrary.MakeVector` (+ _x -100.0) _y _z))))
      (`Pawn.SpawnDefaultController` _returnvalue_2))
    (:`then_2`
      (bind _returnvalue_3 (`|SpawnActorFromClass` "/Game/Blueprints/AI/Swarm_Enemy/SwarmEnemy.SwarmEnemy_C" (`KismetMathLibrary.Conv_VectorToTransform` (`KismetMathLibrary.MakeVector` _x (+ _y 100.0) _z))))
      (`Pawn.SpawnDefaultController` _returnvalue_3))
    (:`then_3`
      (bind _returnvalue_4 (`|SpawnActorFromClass` "/Game/Blueprints/AI/Swarm_Enemy/SwarmEnemy.SwarmEnemy_C" (`KismetMathLibrary.Conv_VectorToTransform` (`KismetMathLibrary.MakeVector` _x (+ _y -100.0) _z))))
      (`Pawn.SpawnDefaultController` _returnvalue_4))))

(fn `UserConstructionScript`)