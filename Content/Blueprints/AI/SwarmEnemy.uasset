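; SwarmEnemy is an AI enemy Blueprint that leaves experience behind when it dies.
; Die destroys the actor, then spawns an ExperienceDrop worth one point at its location with a random rotation and impulse.
; The drop loop has a random count, but the return inside its body ends it after the first drop.
; The shoot function and construction script are empty, with only unwired aiming nodes left over.
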(fn `Die`
  (returns (NewParam :type Boolean))
  (`self.K2_DestroyActor`)
  (for _ (range (+ (`KismetMathLibrary.RandomIntegerInRange` 0 2) 1))
    (bind _returnvalue (`|SpawnActorFromClass` "/Game/Blueprints/ExperienceDrop.ExperienceDrop_C" (`KismetMathLibrary.MakeTransform` (`self.K2_GetActorLocation`) (`KismetMathLibrary.RandomRotator` false))))
    (`PrimitiveComponent.AddImpulse` _returnvalue (* (`KismetMathLibrary.RandomUnitVector`) 500.0) "None" true)
    (`/Game/Blueprints/ExperienceDrop.Set drop value` _returnvalue 1)
    (return false)))

(fn `Swarm enemy shoot`
  (params (`Location to shoot at` :type "Object.Transform Structure")))

(fn `UserConstructionScript`)