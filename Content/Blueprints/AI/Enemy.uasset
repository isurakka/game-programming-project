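; Enemy actor for a co-op game that takes a random color from the CoopGameMode palette on spawn.
; Construction creates and stores a dynamic mesh material, which BeginPlay tints.
; Tick counts down and prints the attack cooldown behind CanAttack, and HealthComponent's OnDie calls Die, a stub returning false.
; The damage flash and hurt sound nodes are disconnected, so AnyDamage does nothing.
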(event `self.ReceiveTick`
  (params (DeltaSeconds :type "Float (single-precision)"))
  (if (> (`self.Attack cooldown`) 0.0)
    (bind _output_get (set `self.Attack cooldown` (- (`self.Attack cooldown`) DeltaSeconds)))
    (`KismetSystemLibrary.PrintString` (`KismetStringLibrary.Conv_DoubleToString` _output_get))))

(event `self.ReceiveBeginPlay`
  (`|ExecutionSequence`
    (:`then_0`
      (bind _ascoop_game_mode (cast `/Game/Blueprints/CoopGameMode` (`GameplayStatics.GetGameMode`))))
    (:`then_1`
      (set `self.ColorIndex` (`KismetMathLibrary.RandomIntegerInRange` 0 (- (`KismetArrayLibrary.Array_Length` (`/Game/Blueprints/CoopGameMode.Colors` _ascoop_game_mode)) 1))))
    (:`then_2`
      (bind _color (`/Game/Blueprints/ColorChangingHelpers.GetColorForIndex` (`self.ColorIndex`) _ascoop_game_mode))
      (bind _asmaterial_instance_dynamic (cast `MaterialInstanceDynamic` (`self.Reference to mesh material`)))
      (`MaterialInstanceDynamic.SetVectorParameterValue` _asmaterial_instance_dynamic "Color" _color))))

(event `self.ReceiveAnyDamage`
  (params (Damage :type "Float (single-precision)") (DamageType :type "DamageType Object Reference") (InstigatedBy :type "Controller Object Reference") (DamageCauser :type "Actor Object Reference")))

(event `self.HealthComponent.OnDie`
  (`self.Die`))

(fn `Can attack`
  (returns (`Can attack` :type Boolean))
  (return (<= (`self.Attack cooldown`) 0.0)))

(fn `Die`
  (returns (NewParam :type Boolean))
  (return false))

(fn `Get world direction`
  (returns (NewParam :type "Object.Vector Structure"))
  (return (`KismetMathLibrary.TransformDirection` (`self.GetTransform`) (1.0 0.0 0.0))))

(fn `ResetMaterial`
  (`PrimitiveComponent.SetMaterial` 0 (`self.Reference to mesh material`)))

(fn `UserConstructionScript`
  (bind _returnvalue (`PrimitiveComponent.CreateDynamicMaterialInstance` 0 (`PrimitiveComponent.GetMaterial` 0)))
  (`PrimitiveComponent.SetMaterial` 0 _returnvalue)
  (set `self.Reference to mesh material` _returnvalue))