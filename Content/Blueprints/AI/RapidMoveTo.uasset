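; RapidMoveTo is a Behavior Tree task that moves a follower AI's pawn toward the actor stored in a blackboard key.
; Execution caches the Follower_AI_CON controller and opens a gate, so Tick reissues AIMoveTo on every frame while it stays open.
; A successful move finishes the task and closes the gate; move failure is not handled.
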(event `self.ReceiveTick`
  (params (OwnerActor :type "Actor Object Reference") (DeltaSeconds :type "Float (single-precision)"))
  (`/Engine/EditorBlueprintResources/StandardMacros.Gate` true :!label _label
    (:`Exit`
      (`|AIMoveTo` (`Controller.K2_GetPawn` (`self.AI_CON_Ref`)) (0.0 0.0 0.0) (`BTFunctionLibrary.GetBlackboardValueAsActor` (`self.TargetToFollow`)) 100.0
        (:`OnSuccess`
          (`self.FinishExecute` true)
          (`self.CloseGate`))))))

(event `self.ReceiveExecute`
  (params (OwnerActor :type "Actor Object Reference"))
  (bind _asfollower_ai_con (cast `/Game/Blueprints/AI/Follower_AI_CON` OwnerActor))
  (set `self.AI_CON_Ref` _asfollower_ai_con)
  (goto _label :!via `Open`))

(event `CloseGate`
  (goto _label :!via `Close`))