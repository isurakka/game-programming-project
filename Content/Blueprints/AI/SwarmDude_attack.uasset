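; Behavior tree task that makes a SwarmEnemy fire at its current blackboard target.
; On execute it casts the owner to Follower_AI_CON and its controlled pawn to SwarmEnemy.
; It reads the TargetToShootAt actor's location, passes it as a transform to SwarmEnemyShoot, then finishes successfully.
; A failed cast stops the graph without calling FinishExecute.
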(event `self.ReceiveExecute`
  (params (OwnerActor :type "Actor Object Reference"))
  (bind _asfollower_ai_con (cast `/Game/Blueprints/AI/Follower_AI_CON` OwnerActor))
  (set `self.AI_CON_Ref` _asfollower_ai_con)
  (bind _asswarm_enemy (cast `/Game/Blueprints/AI/SwarmEnemy` (`Controller.K2_GetPawn` (`self.AI_CON_Ref`))))
  (`/Game/Blueprints/AI/SwarmEnemy.Swarm enemy shoot` _asswarm_enemy (`KismetMathLibrary.Conv_VectorToTransform` (`Actor.K2_GetActorLocation` (`BTFunctionLibrary.GetBlackboardValueAsActor` (`self.TargetToShootAt`)))))
  (`self.FinishExecute` true))