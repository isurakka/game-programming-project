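; FloatingText is an actor that shows text in the world, drifts upward once activated, then fades out and destroys itself.
; It layers an inner and outer text render with settable wording, recolors only the inner one, and gives each a dynamic material instance.
; Activate reveals the text and starts a short fade timer.
; Tick scales the rise by delta time but lowers material opacity by a fixed, frame-rate-dependent step.
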(event `self.ReceiveBeginPlay`)

(event `self.ReceiveActorBeginOverlap`
  (params (OtherActor :type "Actor Object Reference")))

(event `self.ReceiveTick`
  (params (DeltaSeconds :type "Float (single-precision)"))
  (bind _current_opacity (`self.Current opacity`))
  (`|ExecutionSequence`
    (:`then_0`
      (if (`self.Is active`)
        (`self.K2_SetActorLocation` (`KismetMathLibrary.MakeVector` (.x (`self.K2_GetActorLocation`)) (.y (`self.K2_GetActorLocation`)) (+ (.z (`self.K2_GetActorLocation`)) (* DeltaSeconds (`self.Speed`)))))))
    (:`then_1`
      (if (`self.Is fading out`)
        (`MaterialInstanceDynamic.SetScalarParameterValue` (`self.Material instance inner text`) "TextOpacity" _current_opacity)
        (`MaterialInstanceDynamic.SetScalarParameterValue` (`self.Material instance outer text`) "TextOpacity" _current_opacity)
        (bind _output_get (set `self.Current opacity` (- (`self.Current opacity`) 0.02)))
        (if (<= _output_get 0.005)
          (`self.K2_DestroyActor`))))))

(fn `Activate`
  (set `self.Is active` true)
  (`SceneComponent.SetVisibility` (`self.TextRender`) true true)
  (`KismetSystemLibrary.K2_SetTimer` null "Fade Out" 0.5))

(fn `Change text`
  (params (TEXT :type String))
  (`TextRenderComponent.SetText` (`self.TextRender`) TEXT)
  (`TextRenderComponent.SetText` (`self.OuterText`) TEXT))

(fn `Die`)

(fn `Fade out`
  (set `self.Is fading out` true))

(fn `Set color`
  (params (Color :type "Object.LinearColor Structure"))
  (`TextRenderComponent.SetTextRenderColor` (`self.TextRender`) (`KismetMathLibrary.Conv_LinearColorToColor` Color)))

(fn `UserConstructionScript`
  (bind _returnvalue (`PrimitiveComponent.CreateDynamicMaterialInstance` (`self.TextRender`) 0 null))
  (set `self.Material instance inner text` _returnvalue)
  (bind _returnvalue_2 (`PrimitiveComponent.CreateDynamicMaterialInstance` (`self.OuterText`) 0 null))
  (set `self.Material instance outer text` _returnvalue_2))