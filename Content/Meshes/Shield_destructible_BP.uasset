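; Destructible shield Blueprint that can be recolored at runtime and shattered on demand.
; The construction script creates outer and inner dynamic material instances from the Destructible's material slots 1 and 0, though both are created on element index 0.
; SetMaterialDynamicColor writes the Color parameter on each instance.
; Activate breaks the mesh with heavy damage and a randomly directed impulse at the actor's location.
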(event `self.ReceiveBeginPlay`)

(event `self.ReceiveActorBeginOverlap`
  (params (OtherActor :type "Actor Object Reference")))

(event `self.ReceiveTick`
  (params (DeltaSeconds :type "Float (single-precision)")))

(fn `Activate`
  (`DestructibleComponent.ApplyDamage` (`self.Destructible`) 1000.0 (`self.K2_GetActorLocation`) (`KismetMathLibrary.RandomUnitVector`) 5000.0))

(fn `Set material dynamic color`
  (params (`Inner color` :type "Object.LinearColor Structure") (`Outer color` :type "Object.LinearColor Structure"))
  (`|ExecutionSequence`
    (:`then_0`
      (`MaterialInstanceDynamic.SetVectorParameterValue` (`self.inner material`) "Color" `Inner color`))
    (:`then_1`
      (`MaterialInstanceDynamic.SetVectorParameterValue` (`self.outer material`) "Color" `Outer color`))))

(fn `UserConstructionScript`
  (`|ExecutionSequence`
    (:`then_0`
      (bind _returnvalue (`PrimitiveComponent.CreateDynamicMaterialInstance` 0 (`PrimitiveComponent.GetMaterial` (`self.Destructible`) 1)))
      (set `self.outer material` _returnvalue))
    (:`then_1`
      (bind _returnvalue_2 (`PrimitiveComponent.CreateDynamicMaterialInstance` 0 (`PrimitiveComponent.GetMaterial` (`self.Destructible`) 0)))
      (set `self.inner material` _returnvalue_2))))